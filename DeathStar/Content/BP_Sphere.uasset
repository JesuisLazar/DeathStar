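; BP_Sphere is a Blueprint that turns touch drags into controller yaw and pitch input, giving swipe-to-look rotation.
; A touch Moved event records which finger is moving, and Tick polls that finger's state on player controller 0.
; While it stays pressed, the scaled screen-position change since the previous frame drives the rotation.
; A WasTouched flag makes the first pressed frame only store the position, avoiding a jump.
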(event EventTick
  (params (DeltaSeconds :type Float%20%28single-precision%29))
  (bind _returnvalue (Game|GetPlayerController 0))
  (bind _finger_index (Variables|Default|GetFinger%20Index))
  (bind (_locationx _locationy _biscurrentlypressed) (Class|PlayerController|GetInputTouchState _returnvalue _finger_index))
  (if _biscurrentlypressed
    (if (Variables|Default|GetWasTouched)
      (Pawn|Input|AddControllerYawInput (/ (- _locationx (Variables|Default|GetX)) 5.0))
      (Pawn|Input|AddControllerPitchInput (/ (- _locationy (Variables|Default|GetY)) 5.0))
      (Variables|Default|SetX _locationx)
      (Variables|Default|SetY _locationy)
      (else
        (Variables|Default|SetWasTouched true)
        (Variables|Default|SetX _locationx)
        (Variables|Default|SetY _locationy)))
    (else
      (Variables|Default|SetWasTouched false))))

(event Input|TouchEvents|InputTouch
  (params (Location :type Vector) (FingerIndex :type ETouchIndex%20Enum))
  (:Moved
    (Variables|Default|SetFinger%20Index FingerIndex)))

(fn ConstructionScript)