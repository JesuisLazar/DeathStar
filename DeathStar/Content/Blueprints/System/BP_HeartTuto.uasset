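; BP_HeartTuto is the tutorial heart actor, which spawns the WB_Tuto widget and rotates by touch.
; While Tuto is set, Tick turns drags outside the left screen edge into yaw and clamped pitch, notifying the GameInstance.
; Up/Down events snap to twelve preset dodecahedron orientations, and PinchZooming adjusts spring-arm length.
; AnyDamage sets Health to Damage minus Health, then at zero or below plays defeat audio, destroys itself and reports death.
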(event Custom|Down
  ;[1 1 1] WidgetDownDodecahedron
  (Variables|Default|SetRotation "85.000000,170.000000,0.000000")
  (Transformation|SetActorRotation (Variables|Default|GetRotation)))

(event Custom|Down1
  ;[1 1 1] WidgetDownDodecahedron
  (Variables|Default|SetRotation "35.000000,15.000000,0.000000")
  (Transformation|SetActorRotation (Variables|Default|GetRotation)))

(event Custom|Up1
  ;[1 1 1] WidgetUpDodecahedron
  (Variables|Default|SetRotation "-25.000000,55.000000,0.000000")
  (Transformation|SetActorRotation (Variables|Default|GetRotation)))

(event Custom|Up2
  ;[1 1 1] WidgetUpDodecahedron
  (Variables|Default|SetRotation "-25.000000,-15.000000,0.000000")
  (Transformation|SetActorRotation (Variables|Default|GetRotation)))

(event Custom|Up3
  ;[1 1 1] WidgetUpDodecahedron
  (Variables|Default|SetRotation "-25.000000,-85.000000, 0")
  (Transformation|SetActorRotation (Variables|Default|GetRotation)))

(event Custom|Up4
  ;[1 1 1] WidgetUpDodecahedron
  (Variables|Default|SetRotation "-25.000000,-165.000000, 0")
  (Transformation|SetActorRotation (Variables|Default|GetRotation)))

(event Custom|Down2
  ;[1 1 1] WidgetDownDodecahedron
  (Variables|Default|SetRotation "35.000000,-55.000000,0.000000")
  (Transformation|SetActorRotation (Variables|Default|GetRotation)))

(event Custom|Down5
  ;[1 1 1] WidgetDownDodecahedron
  (Variables|Default|SetRotation "35.000000,85.000000, 0")
  (Transformation|SetActorRotation (Variables|Default|GetRotation)))

(event Custom|Down3
  ;[1 1 1] WidgetDownDodecahedron
  (Variables|Default|SetRotation "35.000000,-125.000000, 0")
  (Transformation|SetActorRotation (Variables|Default|GetRotation)))

(event Custom|Down4
  ;[1 1 1] WidgetDownDodecahedron
  (Variables|Default|SetRotation "35.000000,165.000000, 0")
  (Transformation|SetActorRotation (Variables|Default|GetRotation)))

(event Custom|Up5
  ;[1 1 1] WidgetUpDodecahedron
  (Variables|Default|SetRotation "-25.000000,125.000000, 0")
  (Transformation|SetActorRotation (Variables|Default|GetRotation)))

(event Custom|Up
  ;[1 1 1] WidgetUpDodecahedron
  (Variables|Default|SetRotation "-85.000000,-170.000000,0.000000")
  (Transformation|SetActorRotation (Variables|Default|GetRotation)))

(event EventBeginPlay
  ;[1 1 1] MainWidget
  (bind _returnvalue (UserInterface|CreateWidget "/Game/Blueprints/Widget/WB_Tuto.WB_Tuto_C"))
  (bind _output_get (Variables|Default|SetWBMain%20Ref _returnvalue))
  (UserInterface|Viewport|AddtoViewport _output_get 0))

(event Game|Damage|EventAnyDamage
  (params (Damage :type Float%20%28single-precision%29) (DamageType :type Damage%20Type%20Object%20Reference) (InstigatedBy :type Controller%20Object%20Reference) (DamageCauser :type Actor%20Object%20Reference))
  ;[1 1 1] On damage
  (bind _output_get (Variables|Default|SetHealth (- Damage (Variables|Default|GetHealth))))
  (if (<= _output_get 0.0)
    (Audio|PlaySound2D "/Game/Sound/SFX/CUE_Defeat.CUE_Defeat" 1.0 1.0 0.0 0 0)
    (Actor|DestroyActor)
    (Default|CallHearthDead (.AsBP%20Game%20Instance (Utilities|Casting|CastToBP_GameInstance (Game|GetGameInstance))))))

(event EventTick
  (params (DeltaSeconds :type Float%20%28single-precision%29))
  (bind _returnvalue (Game|GetPlayerController 0))
  (bind _fingerindex (Variables|Default|GetFingerIndex))
  (bind (_locationx _locationy _biscurrentlypressed) (Class|PlayerController|GetInputTouchState _returnvalue _fingerindex))
  (bind _returnvalue_2 (> _locationx 8e+01))
  (if (Variables|Default|GetTuto)
    (if _biscurrentlypressed
      (if (not (Variables|Default|GetOnWidget))
        (if (Variables|Default|GetWasTouched)
          (if _returnvalue_2
            (Default|CallTUTOontouch (.AsBP%20Game%20Instance (Utilities|Casting|CastToBP_GameInstance (Game|GetGameInstance))))
            (Pawn|Input|AddControllerYawInput (/ (- _locationx (Variables|Default|GetX)) 1e+01))
            (Variables|Default|SetRotation (Math|Rotator|MakeRotator (.roll (Variables|Default|GetRotation)) (.pitch (Variables|Default|GetRotation)) (+ (* (/ (- _locationx (Variables|Default|GetX)) 1e+01) 2.5) (.yaw (Variables|Default|GetRotation)))))
            (if (and (< (+ (* (/ (- _locationy (Variables|Default|GetY)) 1e+01) -2.5) (.pitch (Variables|Default|GetRotation))) 9e+01) (> (+ (* (/ (- _locationy (Variables|Default|GetY)) 1e+01) -2.5) (.pitch (Variables|Default|GetRotation))) -9e+01))
              (Pawn|Input|AddControllerPitchInput (/ (- _locationy (Variables|Default|GetY)) 1e+01))
              (Variables|Default|SetRotation (Math|Rotator|MakeRotator (.roll (Variables|Default|GetRotation)) (+ (* (/ (- _locationy (Variables|Default|GetY)) 1e+01) -2.5) (.pitch (Variables|Default|GetRotation))) (.yaw (Variables|Default|GetRotation)))))
            (Variables|Default|SetX _locationx)
            (Variables|Default|SetY _locationy)
            (Transformation|SetActorRotation (Variables|Default|GetRotation)))
          (elif _returnvalue_2
            (Variables|Default|SetWasTouched true)
            (Variables|Default|SetX _locationx)
            (Variables|Default|SetY _locationy))))
      (else
        (Variables|Default|SetWasTouched false)))))

(event Input|TouchEvents|InputTouch
  (params (Location :type Vector) (FingerIndex :type ETouchIndex%20Enum))
  (:Moved
    (Variables|Default|SetFingerIndex FingerIndex)))

(fn ConstructionScript)

(fn PinchZooming
  (params (PinchValue :type Float%20%28single-precision%29))
  (bind _springarm (Variables|Default|GetSpringArm))
  (Variables|/Script/Engine.SpringArmComponent|SetTargetArmLength _springarm (Math|Float|Clamp(Float) (+ (Variables|/Script/Engine.SpringArmComponent|GetTargetArmLength _springarm) (* PinchValue (Variables|Default|GetPinchScale))) (Variables|Default|GetZoom%20Min) (Variables|Default|GetZoom%20Max))))