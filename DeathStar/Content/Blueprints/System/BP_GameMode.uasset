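; BP_GameMode is a game mode that tracks wave number and player gold for what appears to be a defence game.
; On BeginPlay it binds handlers to BP_GameInstance start and wave events, each setting the instance's Waves value; the fifth wave's binding is never executed.
; Substract deducts DefencePrice and AddGold adds EnemyPrice, updating both the local Golds and the GameInstance's GoldsOfPlayer.
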(event Custom|Waves1
  (Variables|/Game/Blueprints/System/BP_GameInstance.BP_GameInstance_C|SetWaves (.AsBP%20Game%20Instance (Utilities|Casting|CastToBP_GameInstance (Game|GetGameInstance))) 1))

(event Custom|Substract
  (bind _returnvalue (Game|GetGameInstance))
  (bind _asbp_game_instance (Utilities|Casting|CastToBP_GameInstance _returnvalue))
  (Variables|/Game/Blueprints/System/BP_GameInstance.BP_GameInstance_C|SetGoldsOfPlayer _asbp_game_instance (- (Variables|/Game/Blueprints/System/BP_GameInstance.BP_GameInstance_C|GetGoldsOfPlayer _asbp_game_instance) (Variables|/Game/Blueprints/System/BP_GameInstance.BP_GameInstance_C|GetDefencePrice _asbp_game_instance)))
  (Variables|Default|SetGolds (- (Variables|Default|GetGolds) (Variables|/Game/Blueprints/System/BP_GameInstance.BP_GameInstance_C|GetDefencePrice _asbp_game_instance))))

(event Custom|AddGold
  (bind _returnvalue (Game|GetGameInstance))
  (bind _asbp_game_instance (Utilities|Casting|CastToBP_GameInstance _returnvalue))
  (Variables|Default|SetGolds (+ (Variables|/Game/Blueprints/System/BP_GameInstance.BP_GameInstance_C|GetEnemyPrice _asbp_game_instance) (Variables|Default|GetGolds)))
  (Variables|/Game/Blueprints/System/BP_GameInstance.BP_GameInstance_C|SetGoldsOfPlayer _asbp_game_instance (+ (Variables|/Game/Blueprints/System/BP_GameInstance.BP_GameInstance_C|GetEnemyPrice _asbp_game_instance) (Variables|/Game/Blueprints/System/BP_GameInstance.BP_GameInstance_C|GetGoldsOfPlayer _asbp_game_instance))))

(event Custom|Waves2
  (Variables|/Game/Blueprints/System/BP_GameInstance.BP_GameInstance_C|SetWaves (.AsBP%20Game%20Instance (Utilities|Casting|CastToBP_GameInstance (Game|GetGameInstance))) 2))

(event Custom|Waves3
  (Variables|/Game/Blueprints/System/BP_GameInstance.BP_GameInstance_C|SetWaves (.AsBP%20Game%20Instance (Utilities|Casting|CastToBP_GameInstance (Game|GetGameInstance))) 3))

(event Custom|Waves4
  (Variables|/Game/Blueprints/System/BP_GameInstance.BP_GameInstance_C|SetWaves (.AsBP%20Game%20Instance (Utilities|Casting|CastToBP_GameInstance (Game|GetGameInstance))) 4))

(event Custom|Waves5
  (Variables|/Game/Blueprints/System/BP_GameInstance.BP_GameInstance_C|SetWaves (.AsBP%20Game%20Instance (Utilities|Casting|CastToBP_GameInstance (Game|GetGameInstance))) 5))

(event EventBeginPlay
  (bind _returnvalue (Game|GetGameInstance))
  (bind _asbp_game_instance (Utilities|Casting|CastToBP_GameInstance _returnvalue))
  (EventDispatchers|BindEventtoOnStart _asbp_game_instance (delegate Custom|Waves1))
  (EventDispatchers|BindEventtoWaves2 _asbp_game_instance (delegate Custom|Waves2))
  (EventDispatchers|BindEventtoWaves3 _asbp_game_instance (delegate Custom|Waves3))
  (EventDispatchers|BindEventtoWaves4 _asbp_game_instance (delegate Custom|Waves4)))

(fn ConstructionScript)