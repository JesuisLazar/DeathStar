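; BP_Heart is the player-controlled base core that handles touch input and health, showing the defeat screen and notifying the GameInstance when destroyed.
; A touch manager and joysticks rotate the camera and BP_frame_Blueprint around camera axes, while pinch zooms the spring arm.
; On first start, DoOnce gates step through gesture hints by toggling input locks, though the tutorial widget setup is disconnected.
; It also manages the main HUD and pause menu.
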(event OnXAxisChanged(CameraMovementJoystick)
  (params (Value :type Float%20%28single-precision%29))
  (bind _camera (Variables|Default|GetCamera))
  ;[1 1 1] CameraMovement
  (if (not (Variables|Default|GetTwoFingerOnScreen))
    (if (not (Variables|Tuto|GetLockCamera))
      (Class|Actor|AddActorWorldRotation (Math|Vector|RotatorfromAxisandAngle (Math|Vector|GetUpVector _camera) Value))
      (Class|Actor|AddActorWorldRotation (Math|Vector|RotatorfromAxisandAngle (Math|Vector|GetRightVector _camera) (* (stale OnYAxisChanged(CameraMovementJoystick) Value) -1.0)))
      ;;[1 1 1] Check if is the first Start
      (if (Variables|/Game/Blueprints/System/BP_GameInstance.BP_GameInstance_C|GetFirstStart (.AsBP%20Game%20Instance (Utilities|Casting|CastToBP_GameInstance (Game|GetGameInstance))))
        ;;[1 1 1] Tuto Gesture
        (Utilities|FlowControl|DoOnce false
          (:Completed
            (Utilities|FlowControl|Delay 1.0)
            (Widget|SetVisibility (Variables|/Game/Blueprints/Widget/WB_TutoGesture.WB_TutoGesture_C|GetCameraMovement (Variables|Default|GetWBTutoGestureRef)) "Hidden") ; Cache txt et gif de movement
            (Utilities|FlowControl|Delay 2.0)
            (Widget|SetVisibility (Variables|/Game/Blueprints/Widget/WB_TutoGesture.WB_TutoGesture_C|GetTxtZoom (Variables|Default|GetWBTutoGestureRef)) "Visible") ; Affiche txt et gif de zoom
            (Variables|Tuto|SetLockZoom false) ; Unlock l'input de zoom
          ))))))

(event OnYAxisChanged(CameraMovementJoystick)
  (params (Value :type Float%20%28single-precision%29))
  (bind _camera (Variables|Default|GetCamera))
  ;[1 1 1] CameraMovement
  (if (not (Variables|Default|GetTwoFingerOnScreen))
    (if (not (Variables|Tuto|GetLockCamera))
      (Class|Actor|AddActorWorldRotation (Math|Vector|RotatorfromAxisandAngle (Math|Vector|GetUpVector _camera) (stale OnXAxisChanged(CameraMovementJoystick) Value)))
      (Class|Actor|AddActorWorldRotation (Math|Vector|RotatorfromAxisandAngle (Math|Vector|GetRightVector _camera) (* Value -1.0)))
      ;;[1 1 1] Check if is the first Start
      (if (Variables|/Game/Blueprints/System/BP_GameInstance.BP_GameInstance_C|GetFirstStart (.AsBP%20Game%20Instance (Utilities|Casting|CastToBP_GameInstance (Game|GetGameInstance))))
        ;;[1 1 1] Tuto Gesture
        (Utilities|FlowControl|DoOnce false
          (:Completed
            (Utilities|FlowControl|Delay 1.0)
            (Widget|SetVisibility (Variables|/Game/Blueprints/Widget/WB_TutoGesture.WB_TutoGesture_C|GetCameraMovement (Variables|Default|GetWBTutoGestureRef)) "Hidden") ; Cache txt et gif de movement
            (Utilities|FlowControl|Delay 2.0)
            (Widget|SetVisibility (Variables|/Game/Blueprints/Widget/WB_TutoGesture.WB_TutoGesture_C|GetTxtZoom (Variables|Default|GetWBTutoGestureRef)) "Visible") ; Affiche txt et gif de zoom
            (Variables|Tuto|SetLockZoom false) ; Unlock l'input de zoom
          ))))))

(event OnTwoFingersMove(PinchZoom)
  (params (Zoom :type Float%20%28single-precision%29) (Rotation%20Angle :type Float%20%28single-precision%29) (Initial%20Pan%20Location :type Vector :default "0, 0, 0") (Current%20Pan%20Location :type Vector :default "0, 0, 0") (Pan%20Offset :type Vector :default "0, 0, 0"))
  ;[1 1 1] Zoom
  (if (not (Variables|Tuto|GetLockZoom))
    (Variables|/Script/Engine.SpringArmComponent|SetTargetArmLength (Variables|Default|GetSpringArm) (Math|Float|Clamp(Float) (* Zoom (Variables|Default|GetInitial%20Arm%20Length)) 1.75e+03 3.5e+03))
    ;;[1 1 1] Check if is the first Start
    (if (Variables|/Game/Blueprints/System/BP_GameInstance.BP_GameInstance_C|GetFirstStart (.AsBP%20Game%20Instance (Utilities|Casting|CastToBP_GameInstance (Game|GetGameInstance))))
      ;;[1 1 1] Tuto Gesture
      (Utilities|FlowControl|DoOnce false
        (:Completed
          (Variables|Tuto|SetLockCamera true) ; lock l'input de camera movement
          (Utilities|FlowControl|Delay 1.0)
          (Widget|SetVisibility (Variables|/Game/Blueprints/Widget/WB_TutoGesture.WB_TutoGesture_C|GetTxtZoom (Variables|Default|GetWBTutoGestureRef)) "Hidden") ; Cache txt et gif de zoom
          (Utilities|FlowControl|Delay 2.0)
          (Widget|SetVisibility (Variables|/Game/Blueprints/Widget/WB_TutoGesture.WB_TutoGesture_C|GetBaseRotation (Variables|Default|GetWBTutoGestureRef)) "Visible") ; Affiche txt et gif de rotation
          (Variables|Tuto|SetLockRotation false) ; Unlock l'input de roation
        )))))

(event OnTwoFingersPressed(PinchZoom)
  (params (Pan%20Location :type Vector :default "0, 0, 0"))
  ;[1 1 1] Zoom
  (Variables|Default|SetInitial%20Arm%20Length (Variables|/Script/Engine.SpringArmComponent|GetTargetArmLength (Variables|Default|GetSpringArm)))
  (Variables|Default|SetTwoFingerOnScreen true))

(event OnXAxisChanged(BaseRotationJoystick)
  (params (Value :type Float%20%28single-precision%29))
  (bind _camera (Variables|Default|GetCamera))
  ;[1 1 1] BaseRotation
  (Utilities|FlowControl|Sequence
    (:then_0
      (if (not (Variables|Tuto|GetLockRotation))
        (bind _returnvalue (Actor|GetActorOfClass "/Game/Blueprints/Tiles/BP_frame_Blueprint.BP_frame_Blueprint_C"))
        (Class|Actor|AddActorWorldRotation _returnvalue (Math|Vector|RotatorfromAxisandAngle (Math|Vector|GetUpVector _camera) (* Value -1.0)))
        (Class|Actor|AddActorWorldRotation _returnvalue (Math|Vector|RotatorfromAxisandAngle (Math|Vector|GetRightVector _camera) (stale OnYAxisChanged(BaseRotationJoystick) Value)))
        ;;[1 1 1] Check if is the first Start
        (if (Variables|/Game/Blueprints/System/BP_GameInstance.BP_GameInstance_C|GetFirstStart (.AsBP%20Game%20Instance (Utilities|Casting|CastToBP_GameInstance (Game|GetGameInstance))))
          ;;[1 1 1] Tuto Gesture
          (Utilities|FlowControl|DoOnce false
            (:Completed
              (Variables|Tuto|SetLockZoom true)
              (Utilities|FlowControl|Delay 2.0)
              (Widget|SetVisibility (Variables|/Game/Blueprints/Widget/WB_TutoGesture.WB_TutoGesture_C|GetBaseRotation (Variables|Default|GetWBTutoGestureRef)) "Hidden") ; Cache txt et gif de rotation
              (Utilities|FlowControl|Delay 2.0)
              (Widget|SetVisibility (Variables|/Game/Blueprints/Widget/WB_TutoGesture.WB_TutoGesture_C|GetNext (Variables|Default|GetWBTutoGestureRef)) "Visible"))))))
    (:then_1
      (Utilities|FlowControl|DoOnce false
        (:Completed
          ;;[1 1 1] Hide the Fix jostick
          (Rendering|Material|SetScalarParameterValueonMaterials (Variables|/Script/Engine.StaticMeshActor|GetStaticMeshComponent _returnvalue) "ColorFrame" 1.0))))))

(event OnYAxisChanged(BaseRotationJoystick)
  (params (Value :type Float%20%28single-precision%29))
  (bind _camera (Variables|Default|GetCamera))
  ;[1 1 1] BaseRotation
  (Utilities|FlowControl|Sequence
    (:then_0
      (if (not (Variables|Tuto|GetLockRotation))
        (bind _returnvalue (Actor|GetActorOfClass "/Game/Blueprints/Tiles/BP_frame_Blueprint.BP_frame_Blueprint_C"))
        (Class|Actor|AddActorWorldRotation _returnvalue (Math|Vector|RotatorfromAxisandAngle (Math|Vector|GetUpVector _camera) (* (stale OnXAxisChanged(BaseRotationJoystick) Value) -1.0)))
        (Class|Actor|AddActorWorldRotation _returnvalue (Math|Vector|RotatorfromAxisandAngle (Math|Vector|GetRightVector _camera) Value))
        ;;[1 1 1] Check if is the first Start
        (if (Variables|/Game/Blueprints/System/BP_GameInstance.BP_GameInstance_C|GetFirstStart (.AsBP%20Game%20Instance (Utilities|Casting|CastToBP_GameInstance (Game|GetGameInstance))))
          ;;[1 1 1] Tuto Gesture
          (Utilities|FlowControl|DoOnce false
            (:Completed
              (Variables|Tuto|SetLockZoom true)
              (Utilities|FlowControl|Delay 2.0)
              (Widget|SetVisibility (Variables|/Game/Blueprints/Widget/WB_TutoGesture.WB_TutoGesture_C|GetBaseRotation (Variables|Default|GetWBTutoGestureRef)) "Hidden") ; Cache txt et gif de rotation
              (Utilities|FlowControl|Delay 2.0)
              (Widget|SetVisibility (Variables|/Game/Blueprints/Widget/WB_TutoGesture.WB_TutoGesture_C|GetNext (Variables|Default|GetWBTutoGestureRef)) "Visible"))))))
    (:then_1
      (Utilities|FlowControl|DoOnce false
        (:Completed
          ;;[1 1 1] Hide the Fix jostick
          (Rendering|Material|SetScalarParameterValueonMaterials (Variables|/Script/Engine.StaticMeshActor|GetStaticMeshComponent _returnvalue) "ColorFrame" 1.0))))))

(event OnTwoFingersReleased(PinchZoom)
  (params (Zoom :type Float%20%28single-precision%29) (Rotation%20Angle :type Float%20%28single-precision%29) (Initial%20Pan%20Location :type Vector :default "0, 0, 0") (Current%20Pan%20Location :type Vector :default "0, 0, 0") (Pan%20Offset :type Vector :default "0, 0, 0"))
  ;[1 1 1] Zoom
  (Utilities|FlowControl|Delay 0.1)
  (Variables|Default|SetTwoFingerOnScreen false))

(event OnJoystickPressed(BaseRotationJoystick)
  (params (Location :type Vector :default "0, 0, 0"))
  ;[1 1 1] BaseRotation
  ;;[1 1 1] Hide the Fix jostick
  (Utilities|FlowControl|Sequence
    (:then_0
      (Widget|SetVisibility (Variables|/Game/Blueprints/Widget/WB_Main.WB_Main_C|GetJoystickButton (Variables|Default|GetWBMainRef)) "Hidden"))
    (:then_1
      (Rendering|Material|SetScalarParameterValueonMaterials (Variables|/Script/Engine.StaticMeshActor|GetStaticMeshComponent (stale OnXAxisChanged(BaseRotationJoystick) _returnvalue)) "ColorFrame" 1.0))))

(event OnJoystickReleased(BaseRotationJoystick)
  (params (Location :type Vector :default "0, 0, 0"))
  ;[1 1 1] BaseRotation
  ;;[1 1 1] Hide the Fix jostick
  (Utilities|FlowControl|Sequence
    (:then_0
      (Utilities|FlowControl|Delay 0.5)
      (Widget|SetVisibility (Variables|/Game/Blueprints/Widget/WB_TutoGesture.WB_TutoGesture_C|GetJoystickButton (Variables|Default|GetWBTutoGestureRef)) "Visible"))
    (:then_1
      (Rendering|Material|SetScalarParameterValueonMaterials (Variables|/Script/Engine.StaticMeshActor|GetStaticMeshComponent (stale OnXAxisChanged(BaseRotationJoystick) _returnvalue)) "ColorFrame" 0.0))))

(event Custom|DisplayWidgetAfterTuto
  (bind _baserotationjoystick (Variables|Default|GetBaseRotationJoystick))
  ;[1 1 1] Récupère l'info du dernier Widget tuto pour afficher le main widget
  ;[1 1 1] Display the MainWidget
  (bind _returnvalue (UserInterface|CreateWidget "/Game/Blueprints/Widget/WB_Main.WB_Main_C"))
  (bind _output_get (Variables|Default|SetWBMainRef _returnvalue))
  (UserInterface|Viewport|AddtoViewport _output_get 0)
  ;[1 1 1] Set detection zone of Base Rotation
  (Default|SetupBounds _baserotationjoystick true "(X=140.000000,Y=177.000000)" "(X=150.000000,Y=150.000000)" false false)
  (Variables|/Game/UltimateTouchComponents/Core/UTCComponent.UTCComponent_C|SetPriority _baserotationjoystick 1)
  ;[1 1 1] Display JoystickWidget
  (Default|SetupWidget (Variables|Default|GetBaseRotationJoystick) "/Game/UltimateTouchComponents/AnimatedWidgets/JoystickWidgetAnimated.JoystickWidgetAnimated_C" true false))

(event EventBeginPlay
  (bind _baserotationjoystick (Variables|Default|GetBaseRotationJoystick))
  ;[1 1 1] Récupère l'info du dernier Widget tuto pour afficher le main widget
  (EventDispatchers|BindEventtoDisplayWBMainAftertuto (.AsBP%20Game%20Mode (Utilities|Casting|CastToBP_GameMode (Game|GetGameMode))) (delegate Custom|DisplayWidgetAfterTuto))
  ;[1 1 1] Check if is the first Start
  (if (Variables|/Game/Blueprints/System/BP_GameInstance.BP_GameInstance_C|GetFirstStart (.AsBP%20Game%20Instance (Utilities|Casting|CastToBP_GameInstance (Game|GetGameInstance))))
    _
    (else
      _))
  ;[1 1 1] Display the MainWidget
  (bind _returnvalue (UserInterface|CreateWidget "/Game/Blueprints/Widget/WB_Main.WB_Main_C"))
  (bind _output_get (Variables|Default|SetWBMainRef _returnvalue))
  (UserInterface|Viewport|AddtoViewport _output_get 0)
  ;[1 1 1] Set detection zone of Base Rotation
  (Default|SetupBounds _baserotationjoystick true "(X=140.000000,Y=177.000000)" "(X=150.000000,Y=150.000000)" false false)
  (Variables|/Game/UltimateTouchComponents/Core/UTCComponent.UTCComponent_C|SetPriority _baserotationjoystick 1)
  ;[1 1 1] Display JoystickWidget
  (Default|SetupWidget (Variables|Default|GetBaseRotationJoystick) "/Game/UltimateTouchComponents/AnimatedWidgets/JoystickWidgetAnimated.JoystickWidgetAnimated_C" true false))

(event Game|Damage|EventAnyDamage
  (params (Damage :type Float%20%28single-precision%29) (DamageType :type Damage%20Type%20Object%20Reference) (InstigatedBy :type Controller%20Object%20Reference) (DamageCauser :type Actor%20Object%20Reference))
  ;[1 1 1] On damage
  (bind _output_get (Variables|Default|SetcurrentHealth (- (Variables|Default|GetcurrentHealth) Damage)))
  (if (<= _output_get 0.0)
    (Audio|PlaySound2D "/Game/Sound/SFX/CUE_Defeat.CUE_Defeat" 1.0 1.0 0.0 0 0)
    (Widget|RemovefromParent (Variables|Default|GetWBMainRef))
    (bind _returnvalue (UserInterface|CreateWidget "/Game/Blueprints/Widget/WB_EndGame.WB_EndGame_C"))
    (UserInterface|Viewport|AddtoViewport _returnvalue 0)
    (Default|CallHearthDead (.AsBP%20Game%20Instance (Utilities|Casting|CastToBP_GameInstance (Game|GetGameInstance))))
    (Actor|DestroyActor)))

(event Input|ActionEvents|InputActionPause
  (params (Key :type Key%20Structure :default "None"))
  ;[1 1 1] Pause the Game in PC with Esc
  (:Pressed
    (CallFunction|PauseGame)))

(event Input|TouchEvents|InputTouch
  (params (Location :type Vector) (FingerIndex :type ETouchIndex%20Enum))
  (:Pressed
    ;[1 1 1] Input Touch System
    (Utilities|UTCTouchInputManager Location FingerIndex :!label _label))
  (:Released
    (goto _label Released))
  (:Moved
    (Utilities|FlowControl|Sequence
      (:then_0
        (goto _label Moved))
      (:then_1
        (Default|CallCloseConstructionMenuonMove (.AsBP%20Game%20Mode (Utilities|Casting|CastToBP_GameMode (Game|GetGameMode))))))))

(fn ConstructionScript)

(fn PauseGame
  (Game|SetGamePaused true)
  (Utilities|IsValid (Variables|Default|GetPauseMenu)
    (:Is%20Valid
      _)
    (:Is%20Not%20Valid
      (bind _returnvalue (UserInterface|CreateWidget "/Game/Blueprints/Widget/PauseMenu.PauseMenu_C" (Game|GetPlayerController 0)))
      (bind _output_get (Variables|Default|SetPauseMenu _returnvalue))))
  (UserInterface|Viewport|AddtoViewport _output_get 0)
  (Widget|SetIsEnabled (Variables|Default|GetWBMainRef) false))

(fn UnpauseGame
  (Game|SetGamePaused false)
  (Widget|RemovefromParent (Variables|Default|GetPauseMenu))
  (Widget|SetIsEnabled (Variables|Default|GetWBMainRef) true))