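; Save game object that stores player progression for a turret defense upgrade system.
; A single SaveThis event copies its parameters into matching variables: laser turret health, attack delay modifier and price, plus current and global experience.
; It also records four upgrade levels each for laser, plasma, flak, mortar and space station.
; The graph only assigns values; it contains no disk saving or loading logic.
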(event Custom|SaveThis
  (params (SaveLaserTurretGlobalMaxHealth :type Float%20%28single-precision%29) (SaveLaserTurretGlobalDelayBtwAtkModifier :type Float%20%28single-precision%29) (SaveLaserTurretPrice :type Integer) (SaveExperience :type Integer) (SaveGlobalExperience :type Integer) (SaveLaserUpLvl1 :type Boolean) (SaveLaserUpLvl2 :type Boolean) (SaveLaserUpLvl3 :type Boolean) (SaveLaserUpLvl4 :type Boolean) (SavePlasmaUpLvl1 :type Boolean) (SavePlasmaUpLvl2 :type Boolean) (SavePlasmaUpLvl3 :type Boolean) (SavePlasmaUpLvl4 :type Boolean) (SaveFlakUpLv1 :type Boolean) (SaveFlakUpLv2 :type Boolean) (SaveFlakUpLv3 :type Boolean) (SaveFlakUpLv4 :type Boolean) (SaveMortarUpLv1 :type Boolean) (SaveMortarUpLv2 :type Boolean) (SaveMortarUpLv3 :type Boolean) (SaveMortarUpLv4 :type Boolean) (SaveSpaceStationLv1 :type Boolean) (SaveSpaceStationLv2 :type Boolean) (SaveSpaceStationLv3 :type Boolean) (SaveSpaceStationLv4 :type Boolean))
  (Variables|Default|SetLaserTurretGlobalMaxHealth SaveLaserTurretGlobalMaxHealth)
  (Variables|Default|SetLaserPrice SaveLaserTurretPrice)
  (Variables|Default|SetLaser%20Turret%20Global%20Delay%20Btw%20Atk%20Modifier SaveLaserTurretGlobalDelayBtwAtkModifier)
  (Variables|Default|SetExperience SaveExperience)
  (Variables|Default|SetGlobal%20Experience SaveGlobalExperience)
  (Variables|Default|SetLaserUpLvl1 SaveLaserUpLvl1)
  (Variables|Default|SetLaserUpLvl2 SaveLaserUpLvl2)
  (Variables|Default|SetLaserUpLvl3 SaveLaserUpLvl3)
  (Variables|Default|SetLaserUpLvl4 SaveLaserUpLvl4)
  (Variables|Default|SetPlasmaUpLv1 SavePlasmaUpLvl1)
  (Variables|Default|SetPlasmaUpLvl2 SavePlasmaUpLvl2)
  (Variables|Default|SetPlasmaUpLvl3 SavePlasmaUpLvl3)
  (Variables|Default|SetPlasmaUpLvl4 SavePlasmaUpLvl4)
  (Variables|Default|SetFlakUpLv1 SaveFlakUpLv1)
  (Variables|Default|SetFlakUpLv2 SaveFlakUpLv2)
  (Variables|Default|SetFlakUpLv3 SaveFlakUpLv3)
  (Variables|Default|SetFlakUpLv4 SaveFlakUpLv4)
  (Variables|Default|SetMortarUpLv1 SaveMortarUpLv1)
  (Variables|Default|SetMortarUpLv2 SaveMortarUpLv2)
  (Variables|Default|SetMortarUpLv3 SaveMortarUpLv3)
  (Variables|Default|SetMortarUpLv4 SaveMortarUpLv4)
  (Variables|Default|SetSpaceStationLv1 SaveSpaceStationLv1)
  (Variables|Default|SetSpaceStationLv2 SaveSpaceStationLv2)
  (Variables|Default|SetSpaceStationLv3 SaveSpaceStationLv3)
  (Variables|Default|SetSpaceStationLv4 SaveSpaceStationLv4))