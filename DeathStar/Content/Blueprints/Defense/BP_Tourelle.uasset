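; BP_Tourelle is a defense turret that damages enemies inside its detection box and destroys itself when its health runs out.
; BeginPlay sizes and offsets the box from the depth, width and height variables.
; Overlaps maintain a list of BP_Enemyy; a DoOnce starts a looping one-second timer, cleared and reset when the list empties.
; Each tick of that timer subtracts Damage directly from the first listed enemy's Health.
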(event OnComponentBeginOverlap(Box)
  (params (OverlappedComponent :type Primitive%20Component%20Object%20Reference) (OtherActor :type Actor%20Object%20Reference) (OtherComp :type Primitive%20Component%20Object%20Reference) (OtherBodyIndex :type Integer) (bFromSweep :type Boolean) (SweepResult :type Hit%20Result%20Structure%20%28by%20ref%29))
  ;[1 1 1] Setting Array for Enemy and giving damage
  (bind _asbp_enemyy (Utilities|Casting|CastToBP_Enemyy OtherActor))
  (Utilities|Array|Add (Variables|Default|GetListOfEnemy1) _asbp_enemyy)
  (Utilities|FlowControl|DoOnce false
    (:Completed
      (Utilities|Time|SetTimerbyFunctionName 0 "AttackEnemy1" 1.0 true))))

(event OnComponentEndOverlap(Box)
  (params (OverlappedComponent :type Primitive%20Component%20Object%20Reference) (OtherActor :type Actor%20Object%20Reference) (OtherComp :type Primitive%20Component%20Object%20Reference) (OtherBodyIndex :type Integer))
  ;[1 1 1] Setting Array for Enemy and giving damage
  (bind _asbp_enemyy (Utilities|Casting|CastToBP_Enemyy OtherActor))
  (Utilities|Array|RemoveItem (Variables|Default|GetListOfEnemy1) _asbp_enemyy)
  (if (== (Utilities|Array|Length (Variables|Default|GetListOfEnemy1)) 0)
    (Utilities|Time|ClearTimerbyFunctionName 0 "AttackEnemy1")
    (Utilities|FlowControl|DoOnce false) ; enters at Reset
  ))

(event EventBeginPlay
  (bind _depthboxdetection (Variables|Default|GetDepthBoxDetection))
  ;[1 1 1] Setting Box Damage Collision
  (Transformation|AddLocalOffset (Variables|Default|GetBox) (Math|Vector|MakeVector _depthboxdetection 0.0 0.0) false false)
  (Components|Box|SetBoxExtent (Variables|Default|GetBox) (Math|Vector|MakeVector _depthboxdetection (Variables|Default|GetWidthBoxDetection) (Variables|Default|GetHeightBoxDetection)) true))

(event Game|Damage|EventAnyDamage
  (params (Damage :type Float%20%28single-precision%29) (DamageType :type Damage%20Type%20Object%20Reference) (InstigatedBy :type Controller%20Object%20Reference) (DamageCauser :type Actor%20Object%20Reference))
  ;[1 1 1] Taking Damage from Enemy
  (bind _output_get (Variables|Default|SetHealth (- (Variables|Default|GetHealth) Damage)))
  (if (<= _output_get 0.0)
    (Actor|DestroyActor)))

(fn ConstructionScript)

(fn AttackEnemy1
  (bind _listofenemy1 (Variables|Default|GetListOfEnemy1))
  (bind _output (Utilities|Array|Get(acopy) _listofenemy1))
  (Variables|/Game/Blueprints/Enemy/BP_Enemyy.BP_Enemyy_C|SetHealth _output (- (Variables|/Game/Blueprints/Enemy/BP_Enemyy.BP_Enemyy_C|GetHealth _output) (Variables|Default|GetDamage))))