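; BPC_LaserTutorial is a defense actor Blueprint, by its name the tutorial version of a laser turret, with a turret life widget.
; On BeginPlay it casts its widget component's UI to UI_LifeTurret, hands it a self reference, then calls the parent BeginPlay, which is skipped if the cast fails.
; Tick and construction only forward to the parent, and the overlap event is disabled.
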(event EventBeginPlay
  (bind _asui_life_turret (Utilities|Casting|CastToUI_LifeTurret (UserInterface|GetUserWidgetObject (Variables|Default|GetWidget_0))))
  (Variables|/Game/Blueprints/Widget/UI_LifeTurret.UI_LifeTurret_C|SetActor _asui_life_turret self)
  (|CallParentFunction))

(event Collision|EventActorBeginOverlap
  (params (OtherActor :type Actor%20Object%20Reference))
  (|CallParentFunction OtherActor) ; This node is disabled and will not be called.\nDrag off pins to build functionality.
)

(event EventTick
  (params (DeltaSeconds :type Float%20%28single-precision%29))
  (|CallParentFunction DeltaSeconds))

(fn ConstructionScript
  (|CallParentFunction))