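; Flak turret for the defense game, a child turret Blueprint that fires flak projectiles.
; BeginPlay loads its stats and price from BP_GameInstance, binds to the GameMode's turret-upgrade event and sets up the life widget, laser sight and crosshair.
; When selected, it takes two one-shot upgrade tiers that adjust stats, range and visuals, then deduct Materials.
; Touches on its meshes notify the GameInstance to disable camera rotation.
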(event OnInputTouchBegin(TurretTop)
  (params (FingerIndex :type ETouchIndex%20Enum :default "Touch1") (TouchedComponent :type Primitive%20Component%20Object%20Reference))
  ;[1 1 1] Call the Event when is touch for disable Camera rotation
  (bind _asbp_game_instance (Utilities|Casting|CastToBP_GameInstance (Game|GetGameInstance)))
  (Default|CallBaseTouched _asbp_game_instance))

(event OnInputTouchBegin(Plane1)
  (params (FingerIndex :type ETouchIndex%20Enum :default "Touch1") (TouchedComponent :type Primitive%20Component%20Object%20Reference))
  ;[1 1 1] Call the Event when is touch for disable Camera rotation
  (bind _asbp_game_instance (Utilities|Casting|CastToBP_GameInstance (Game|GetGameInstance)))
  (Default|CallBaseTouched _asbp_game_instance))

(event OnInputTouchBegin(Mesh_Flak)
  (params (FingerIndex :type ETouchIndex%20Enum :default "Touch1") (TouchedComponent :type Primitive%20Component%20Object%20Reference))
  ;[1 1 1] Call the Event when is touch for disable Camera rotation
  (bind _asbp_game_instance (Utilities|Casting|CastToBP_GameInstance (Game|GetGameInstance)))
  (Default|CallBaseTouched _asbp_game_instance))

(event Custom|UpgradeFlak
  (bind _returnvalue (Game|GetGameMode))
  (bind _returnvalue_2 (Game|Player|GetPlayerPawn 0))
  (bind _outlinetop (Variables|Default|GetOutlineTop))
  (bind _turrettop (Variables|Default|GetTurretTop))
  (bind _outlinetop_2 (Variables|Default|GetOutlineTop))
  (bind _turrettop_2 (Variables|Default|GetTurretTop))
  (bind _turret_aura_upgrade_system (Variables|Default|Getturret_aura_upgrade_System))
  (bind _asbp_game_mode (Utilities|Casting|CastToBP_GameMode _returnvalue))
  (bind _asbp_heart (Utilities|Casting|CastToBP_Heart _returnvalue_2))
  (bind _wbmainref (Variables|/Game/Blueprints/System/BP_Heart.BP_Heart_C|GetWBMainRef _asbp_heart))
  (if (Variables|Default|GetSelected)
    (if (Variables|Default|GethasBeenUpgradedOnce)
      (Utilities|FlowControl|DoOnce false
        (:Completed
          ;[1 1 1] Upgrade 2
          (Utilities|FlowControl|Sequence
            (:then_1
              (bind _output_get (Variables|Default|SetDelayBtwAtk (+ (Variables|Default|GetDelayBtwAtk) 0.05)))
              ;;[0.03022 1 0] Debug
              (Development|PrintString (Utilities|String|ToString(Float) _output_get)))
            (:then_2
              (bind _output_get_2 (Variables|Default|SetMaxHealth (+ (Variables|Default|GetMaxHealth) 3e+01)))
              (Development|PrintString (Utilities|String|ToString(Float) _output_get_2)))
            (:then_3
              (Variables|Default|SetHealth (+ (Variables|Default|GetHealth) 3e+01)))
            (:then_4
              (Transformation|SetWorldScale3D (Variables|Default|GetDetectionArea) (Math|Vector|MakeVector (+ (Variables|Default|GetScaleX) 2.0) (+ (Variables|Default|GetScaleY) 2.0) (+ (Variables|Default|GetScaleZ) 2.0)))
              ;;[0.03022 1 0] Debug
              (Development|PrintString "SCALEUP2")
              (Variables|Default|SetScaleZ (+ (Variables|Default|GetScaleZ) 2.0))
              (Variables|Default|SetRange (+ (Variables|Default|GetScaleZ) 2.0)))
            (:then_5
              (Audio|PlaySound2D "/Game/Sound/TurretSFX/SFX_UpgradeCompleted.SFX_UpgradeCompleted" 1.0 1.2 0.0 0 0)
              ;;[0.03022 1 0] Debug
              (Development|PrintString "UPGRADE 2")
              (Variables|Default|SethasBeenUpgradedtwice true)
              (Widget|SetVisibility (Variables|/Game/Blueprints/Widget/WB_Main.WB_Main_C|GetUpgrade _wbmainref) "Hidden")
              ;[1 1 1] Substract the cost of upgrade to Materials
              (Variables|/Game/Blueprints/System/BP_GameMode.BP_GameMode_C|SetMaterials _asbp_game_mode (- (Variables|/Game/Blueprints/System/BP_GameMode.BP_GameMode_C|GetMaterials _asbp_game_mode) (Variables|/Game/Blueprints/Widget/WB_Main.WB_Main_C|GetUpgradeCostTxt _wbmainref)) :!label _label))
            (:then_6
              (Transformation|SetWorldScale3D _outlinetop (+ (Transformation|GetWorldScale _outlinetop) "0.050000,0.050000,0.050000"))
              (Transformation|SetWorldScale3D _turrettop (+ (Transformation|GetWorldScale _turrettop) "0.050000,0.050000,0.050000")))
            (:then_7
              (Niagara|SetNiagaraVariable(Float) (Variables|Default|Getturret_aura_upgrade_System) "Uniform Sprite Size" 6e+01)))))
      (else
        (Utilities|FlowControl|DoOnce false
          (:Completed
            ;[1 1 1] Upgrade 1
            (Utilities|FlowControl|Sequence
              (:then_0
                (bind _output_get_3 (Variables|Default|SetDamage (+ (Variables|Default|GetDamage) 2.0)))
                ;;[0.03022 1 0] Debug
                (Development|PrintString (Utilities|String|ToString(Float) _output_get_3)))
              (:then_1
                (bind _output_get_4 (Variables|Default|SetDelayBtwAtk (+ (Variables|Default|GetDelayBtwAtk) 0.05)))
                (Development|PrintString (Utilities|String|ToString(Float) _output_get_4)))
              (:then_2
                (bind _output_get_5 (Variables|Default|SetMaxHealth (+ (Variables|Default|GetMaxHealth) 3e+01)))
                (Development|PrintString (Utilities|String|ToString(Float) _output_get_5)))
              (:then_3
                (Variables|Default|SetHealth (+ (Variables|Default|GetHealth) 3e+01)))
              (:then_4
                (Transformation|SetWorldScale3D (Variables|Default|GetDetectionArea) (Math|Vector|MakeVector (+ (Variables|Default|GetScaleX) 1.0) (+ (Variables|Default|GetScaleY) 1.0) (+ (Variables|Default|GetScaleZ) 1.0)))
                (Variables|Default|SetScaleZ (+ (Variables|Default|GetScaleZ) 1.0))
                (Variables|Default|SetRange (+ (Variables|Default|GetScaleZ) 1.0)))
              (:then_5
                (Audio|PlaySound2D "/Game/Sound/TurretSFX/SFX_UpgradeCompleted.SFX_UpgradeCompleted" 1.0 1.0 0.0 0 0)
                ;;[0.03022 1 0] Debug
                (Development|PrintString "UPGRADE 1")
                (Variables|Default|SethasBeenUpgradedOnce true)
                (goto _label))
              (:then_6
                (Transformation|SetWorldScale3D _outlinetop_2 (+ (Transformation|GetWorldScale _outlinetop_2) "0.050000,0.050000,0.050000"))
                (Transformation|SetWorldScale3D _turrettop_2 (+ (Transformation|GetWorldScale _turrettop_2) "0.050000,0.050000,0.050000")))
              (:then_7
                ;;[1 1 1] Aura Upgrade Color & Size
                (Niagara|SetNiagaraVariable(Vector3) _turret_aura_upgrade_system "Scale RGB" (Math|Conversions|ToVector(LinearColor) (Variables|Default|GetauraUpgradeColor)))
                (Niagara|SetNiagaraVariable(Float) _turret_aura_upgrade_system "Uniform Sprite Size" 5e+01)))))))))

(event EventBeginPlay
  (bind _crosshair (Variables|Default|GetCrosshair))
  (Variables|Default|SetdamageFeedbackColor "(R=0.000000,G=0.000000,B=50.000000,A=1.000000)")
  (Variables|Default|SetisFlak true)
  (Variables|Default|SetclassProjectile "/Game/VFX/TurretVFX/TurretRoundsNiagara/BP_TurretProjectiles_Flak.BP_TurretProjectiles_Flak_C")
  (Utilities|FlowControl|Sequence
    (:then_0
      (CallFunction|SetGameInstanceValue)
      (EventDispatchers|BindEventtoAllTurretUpgrade (.AsBP%20Game%20Mode (Utilities|Casting|CastToBP_GameMode (Game|GetGameMode))) (delegate Custom|UpgradeFlak))
      (bind _asui_life_turret (Utilities|Casting|CastToUI_LifeTurret (UserInterface|GetUserWidgetObject (Variables|Default|GetWidget))))
      (Variables|/Game/Blueprints/Widget/UI_LifeTurret.UI_LifeTurret_C|SetActor _asui_life_turret self)
      (|CallParentFunction))
    (:then_1
      (Niagara|SetNiagaraVariable(LinearColor) (Variables|Default|GetLasersight) "User.BeamColor" (Variables|Default|GetbeamColor))
      (Niagara|SetNiagaraVariable(Vector3) _crosshair "Scale RGB" (Math|Conversions|ToVector(LinearColor) (Variables|Default|GettargetColor)))
      (Niagara|SetNiagaraVariable(Float) _crosshair "Uniform Sprite Size" 8e+02)
      (Niagara|SetNiagaraVariable(Vector3) _crosshair "Position Offset" "0.300000, 0, 0"))))

(event Collision|EventActorBeginOverlap
  (params (OtherActor :type Actor%20Object%20Reference))
  (|CallParentFunction OtherActor) ; This node is disabled and will not be called.\nDrag off pins to build functionality.
)

(event EventTick
  (params (DeltaSeconds :type Float%20%28single-precision%29))
  (|CallParentFunction DeltaSeconds))

(fn ConstructionScript
  (|CallParentFunction))

(fn SetGameInstanceValue
  (bind _returnvalue (Game|GetGameInstance))
  (bind _asbp_game_instance (Utilities|Casting|CastToBP_GameInstance _returnvalue))
  (Variables|Default|SetDamage (Variables|/Game/Blueprints/System/BP_GameInstance.BP_GameInstance_C|GetFlakTurretGlobalDamageModifier _asbp_game_instance))
  (Variables|Default|SetDelayBtwAtk (Variables|/Game/Blueprints/System/BP_GameInstance.BP_GameInstance_C|GetFlakTurretGlobalDelayBtwAtkModifier _asbp_game_instance))
  (Variables|Default|SetScaleZ (Variables|/Game/Blueprints/System/BP_GameInstance.BP_GameInstance_C|GetFlakTurretGlobalRangeModifier _asbp_game_instance))
  (Variables|Default|SetMaxHealth (Variables|/Game/Blueprints/System/BP_GameInstance.BP_GameInstance_C|GetFlakTurretGlobalMaxHealthModifier _asbp_game_instance))
  (Variables|Default|SetHealth (Variables|/Game/Blueprints/System/BP_GameInstance.BP_GameInstance_C|GetFlakTurretGlobalActualHealthModifier _asbp_game_instance))
  (Variables|Default|SetPrice (Variables|/Game/Blueprints/System/BP_GameInstance.BP_GameInstance_C|GetflakTurretPrice _asbp_game_instance)))