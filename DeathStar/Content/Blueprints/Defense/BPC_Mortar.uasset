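; Mortar turret for a defense game, a child Blueprint that sets the mortar projectile class and adds mortar-specific stats and upgrades.
; On BeginPlay it loads stats from the GameInstance, binds to the GameMode's upgrade event and links its life widget before running parent logic.
; When selected, it upgrades through two one-shot tiers, boosting stats and splash radius and deducting Materials.
; Touching the mesh or plane notifies the GameInstance to disable camera rotation.
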(event OnInputTouchBegin(Mesh_Mortar)
  (params (FingerIndex :type ETouchIndex%20Enum :default "Touch1") (TouchedComponent :type Primitive%20Component%20Object%20Reference))
  ;[1 1 1] Call the Event when is touch for disable Camera rotation
  (bind _asbp_game_instance (Utilities|Casting|CastToBP_GameInstance (Game|GetGameInstance)))
  (Default|CallBaseTouched _asbp_game_instance))

(event OnInputTouchBegin(Plane1)
  (params (FingerIndex :type ETouchIndex%20Enum :default "Touch1") (TouchedComponent :type Primitive%20Component%20Object%20Reference))
  ;[1 1 1] Call the Event when is touch for disable Camera rotation
  (bind _asbp_game_instance (Utilities|Casting|CastToBP_GameInstance (Game|GetGameInstance)))
  (Default|CallBaseTouched _asbp_game_instance))

(event Custom|UpgradeMortar
  (bind _returnvalue (Game|GetGameMode))
  (bind _returnvalue_2 (Game|Player|GetPlayerPawn 0))
  (bind _splashdamagecollisionsphere (Variables|Default|GetsplashDamageCollisionSphere))
  (bind _splashdamagecollisionsphere_2 (Variables|Default|GetsplashDamageCollisionSphere))
  (bind _asbp_game_mode (Utilities|Casting|CastToBP_GameMode _returnvalue))
  (bind _asbp_heart (Utilities|Casting|CastToBP_Heart _returnvalue_2))
  (bind _wbmainref (Variables|/Game/Blueprints/System/BP_Heart.BP_Heart_C|GetWBMainRef _asbp_heart))
  (if (Variables|Default|GetSelected)
    (if (Variables|Default|GethasBeenUpgradedOnce)
      (Utilities|FlowControl|DoOnce false
        (:Completed
          ;[1 1 1] Upgrade 2
          (Utilities|FlowControl|Sequence
            (:then_1
              (bind _output_get (Variables|Default|SetDelayBtwAtk (+ (Variables|Default|GetDelayBtwAtk) -0.25)))
              ;;[0.03022 1 0] Debug
              (Development|PrintString (Utilities|String|ToString(Float) _output_get)))
            (:then_2
              (bind _output_get_2 (Variables|Default|SetMaxHealth (+ (Variables|Default|GetMaxHealth) 8e+01)))
              (Development|PrintString (Utilities|String|ToString(Float) _output_get_2)))
            (:then_3
              (Variables|Default|SetHealth (+ (Variables|Default|GetHealth) 8e+01)))
            (:then_4
              (Transformation|SetWorldScale3D (Variables|Default|GetDetectionArea) (Math|Vector|MakeVector (+ (Variables|Default|GetScaleX) 2.0) (+ (Variables|Default|GetScaleY) 2.0) (+ (Variables|Default|GetScaleZ) 2.0)))
              ;;[0.03022 1 0] Debug
              (Development|PrintString "SCALEUP2")
              (Variables|Default|SetScaleZ (+ (Variables|Default|GetScaleZ) 2.0))
              (Variables|Default|SetRange (+ (Variables|Default|GetScaleZ) 2.0)))
            (:then_5
              (Components|Sphere|SetSphereRadius _splashdamagecollisionsphere_2 (+ (Variables|/Script/Engine.SphereComponent|GetSphereRadius _splashdamagecollisionsphere_2) 5e+01) true))
            (:then_6
              (Audio|PlaySound2D "/Game/Sound/TurretSFX/SFX_UpgradeCompleted.SFX_UpgradeCompleted" 1.0 1.2 0.0 0 0)
              ;;[0.03022 1 0] Debug
              (Development|PrintString "UPGRADE 2")
              (Variables|Default|SethasBeenUpgradedtwice true)
              (Widget|SetVisibility (Variables|/Game/Blueprints/Widget/WB_Main.WB_Main_C|GetUpgrade _wbmainref) "Hidden")
              ;[1 1 1] Substract the cost of upgrade to Materials
              (Variables|/Game/Blueprints/System/BP_GameMode.BP_GameMode_C|SetMaterials _asbp_game_mode (- (Variables|/Game/Blueprints/System/BP_GameMode.BP_GameMode_C|GetMaterials _asbp_game_mode) (Variables|/Game/Blueprints/Widget/WB_Main.WB_Main_C|GetUpgradeCostTxt _wbmainref)) :!label _label)))))
      (else
        (Utilities|FlowControl|DoOnce false
          (:Completed
            ;[1 1 1] Upgrade 1
            (Utilities|FlowControl|Sequence
              (:then_0
                (bind _output_get_3 (Variables|Default|SetDamage (+ (Variables|Default|GetDamage) 12.0)))
                ;;[0.03022 1 0] Debug
                (Development|PrintString (Utilities|String|ToString(Float) _output_get_3)))
              (:then_1
                (bind _output_get_4 (Variables|Default|SetDelayBtwAtk (+ (Variables|Default|GetDelayBtwAtk) -0.25)))
                (Development|PrintString (Utilities|String|ToString(Float) _output_get_4)))
              (:then_2
                (bind _output_get_5 (Variables|Default|SetMaxHealth (+ (Variables|Default|GetMaxHealth) 8e+01)))
                (Development|PrintString (Utilities|String|ToString(Float) _output_get_5)))
              (:then_3
                (Variables|Default|SetHealth (+ (Variables|Default|GetHealth) 8e+01)))
              (:then_4
                (Transformation|SetWorldScale3D (Variables|Default|GetDetectionArea) (Math|Vector|MakeVector (+ (Variables|Default|GetScaleX) 1.0) (+ (Variables|Default|GetScaleY) 1.0) (+ (Variables|Default|GetScaleZ) 1.0)))
                (Variables|Default|SetScaleZ (+ (Variables|Default|GetScaleZ) 1.0))
                (Variables|Default|SetRange (+ (Variables|Default|GetScaleZ) 1.0)))
              (:then_5
                (Components|Sphere|SetSphereRadius _splashdamagecollisionsphere (+ (Variables|/Script/Engine.SphereComponent|GetSphereRadius _splashdamagecollisionsphere) 5e+01) true))
              (:then_6
                (Audio|PlaySound2D "/Game/Sound/TurretSFX/SFX_UpgradeCompleted.SFX_UpgradeCompleted" 1.0 1.0 0.0 0 0)
                ;;[0.03022 1 0] Debug
                (Development|PrintString "UPGRADE 1")
                (Variables|Default|SethasBeenUpgradedOnce true)
                (goto _label)))))))))

(event EventBeginPlay
  (Variables|Default|SetisMortar true)
  (Variables|Default|SetclassProjectile "/Game/VFX/TurretVFX/TurretRoundsNiagara/BP_TurretProjectiles_Mortar.BP_TurretProjectiles_Mortar_C")
  (CallFunction|SetGameInstanceValue)
  (EventDispatchers|BindEventtoAllTurretUpgrade (.AsBP%20Game%20Mode (Utilities|Casting|CastToBP_GameMode (Game|GetGameMode))) (delegate Custom|UpgradeMortar))
  (bind _asui_life_turret (Utilities|Casting|CastToUI_LifeTurret (UserInterface|GetUserWidgetObject (Variables|Default|GetWidget))))
  (Variables|/Game/Blueprints/Widget/UI_LifeTurret.UI_LifeTurret_C|SetActor _asui_life_turret self)
  (|CallParentFunction))

(fn ConstructionScript
  (|CallParentFunction))

(fn SetGameInstanceValue
  (bind _returnvalue (Game|GetGameInstance))
  (bind _asbp_game_instance (Utilities|Casting|CastToBP_GameInstance _returnvalue))
  (bind _mortarturretglobalrangemodifier (Variables|/Game/Blueprints/System/BP_GameInstance.BP_GameInstance_C|GetMortarTurretGlobalRangeModifier _asbp_game_instance))
  (Variables|Default|SetDamage (Variables|/Game/Blueprints/System/BP_GameInstance.BP_GameInstance_C|GetMortarTurretGlobalDamageModifier _asbp_game_instance))
  (Variables|Default|SetDelayBtwAtk (Variables|/Game/Blueprints/System/BP_GameInstance.BP_GameInstance_C|GetMortarTurretGlobalDelayBtwAtkModifier _asbp_game_instance))
  (Variables|Default|SetScaleX _mortarturretglobalrangemodifier)
  (Variables|Default|SetScaleY _mortarturretglobalrangemodifier)
  (Variables|Default|SetScaleZ _mortarturretglobalrangemodifier)
  (Variables|Default|SetMaxHealth (Variables|/Game/Blueprints/System/BP_GameInstance.BP_GameInstance_C|GetMortarTurretGlobalMaxHealthModifier _asbp_game_instance))
  (Variables|Default|SetHealth (Variables|/Game/Blueprints/System/BP_GameInstance.BP_GameInstance_C|GetMortarTurretGlobalActualHealthModifier _asbp_game_instance))
  (Variables|Default|SetPrice (Variables|/Game/Blueprints/System/BP_GameInstance.BP_GameInstance_C|GetmortarTurretPrice _asbp_game_instance))
  (Variables|Default|SetturretArmor (Variables|/Game/Blueprints/System/BP_GameInstance.BP_GameInstance_C|GetMortarTurretGlobalArmor _asbp_game_instance))
  (Components|Sphere|SetSphereRadius (Variables|Default|GetsplashDamageCollisionSphere) (Variables|/Game/Blueprints/System/BP_GameInstance.BP_GameInstance_C|GetMortarTurretGlobalProjectileRadius _asbp_game_instance) true))