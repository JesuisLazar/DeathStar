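; Laser defense Blueprint that shows a turret life widget and passes touches through to base selection.
; On BeginPlay it hands itself to the UI_LifeTurret in its widget component, then runs the parent's BeginPlay.
; Touches on the Laser and Plane1 components call CallBaseSelected on BP_GameInstance, so they act as a tap on the base.
; Tick and construction only defer to the parent class.
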(event OnInputTouchBegin(Plane1)
  (params (FingerIndex :type ETouchIndex%20Enum :default "Touch1") (TouchedComponent :type Primitive%20Component%20Object%20Reference))
  ;[1 1 1] Touch go through
  (bind _asbp_game_instance (Utilities|Casting|CastToBP_GameInstance (Game|GetGameInstance)))
  (Default|CallBaseSelected _asbp_game_instance))

(event OnInputTouchBegin(Laser)
  (params (FingerIndex :type ETouchIndex%20Enum :default "Touch1") (TouchedComponent :type Primitive%20Component%20Object%20Reference))
  ;[1 1 1] Touch go through
  (bind _asbp_game_instance (Utilities|Casting|CastToBP_GameInstance (Game|GetGameInstance)))
  (Default|CallBaseSelected _asbp_game_instance))

(event EventBeginPlay
  (bind _asui_life_turret (Utilities|Casting|CastToUI_LifeTurret (UserInterface|GetUserWidgetObject (Variables|Default|GetWidget))))
  (Variables|/Game/Blueprints/Widget/UI_LifeTurret.UI_LifeTurret_C|SetActor _asui_life_turret self)
  (|CallParentFunction))

(event Collision|EventActorBeginOverlap
  (params (OtherActor :type Actor%20Object%20Reference))
  (|CallParentFunction OtherActor) ; This node is disabled and will not be called.\nDrag off pins to build functionality.
)

(event EventTick
  (params (DeltaSeconds :type Float%20%28single-precision%29))
  (|CallParentFunction DeltaSeconds))

(fn ConstructionScript
  (|CallParentFunction))