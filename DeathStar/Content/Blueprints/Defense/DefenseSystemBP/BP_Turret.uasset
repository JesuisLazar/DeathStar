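; Defense turret actor that shoots BP_Enemyy actors inside a forward box, which it sizes and offsets by Range on BeginPlay.
; Overlaps maintain an enemy list; the first entry starts casting and repeating attack timers through a DoOnce, both reset when the list empties.
; AttackEnemy subtracts HP directly from the oldest listed enemy, with two muzzle effects and a shot sound.
; Incoming damage lowers Health, destroying the turret with a sound at zero.
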(event OnComponentBeginOverlap(Box)
  (params (OverlappedComponent :type Primitive%20Component%20Object%20Reference) (OtherActor :type Actor%20Object%20Reference) (OtherComp :type Primitive%20Component%20Object%20Reference) (OtherBodyIndex :type Integer) (bFromSweep :type Boolean) (SweepResult :type Hit%20Result%20Structure%20%28by%20ref%29))
  ;[1 1 1] Setting Array for Enemy and giving damage
  (bind _asbp_enemyy (Utilities|Casting|CastToBP_Enemyy OtherActor))
  (Utilities|Array|Add (Variables|Default|GetListOfEnemy1) _asbp_enemyy)
  (Utilities|FlowControl|DoOnce false
    (:Completed
      (Utilities|Time|SetTimerbyFunctionName 0 "AttackEnemy" (Variables|Default|GetCastingTime))
      (Utilities|FlowControl|Delay 0.1)
      (Utilities|Time|SetTimerbyFunctionName 0 "AttackEnemy" (Variables|Default|GetDelayBtwAtk) true))))

(event OnComponentEndOverlap(Box)
  (params (OverlappedComponent :type Primitive%20Component%20Object%20Reference) (OtherActor :type Actor%20Object%20Reference) (OtherComp :type Primitive%20Component%20Object%20Reference) (OtherBodyIndex :type Integer))
  ;[1 1 1] Setting Array for Enemy and giving damage
  (bind _asbp_enemyy (Utilities|Casting|CastToBP_Enemyy OtherActor))
  (Utilities|Array|RemoveItem (Variables|Default|GetListOfEnemy1) _asbp_enemyy)
  (if (== (Utilities|Array|Length (Variables|Default|GetListOfEnemy1)) 0)
    ;;[1 1 1] A CHECK AVEC AUREL
    (Utilities|FlowControl|Delay 0.01)
    (Utilities|Time|ClearTimerbyFunctionName 0 "AttackEnemy")
    (Utilities|FlowControl|DoOnce false) ; enters at Reset
  ))

(event EventBeginPlay
  (bind _range (Variables|Default|GetRange))
  ;[1 1 1] Setting Box Damage Collision
  (Utilities|FlowControl|Sequence
    (:then_0
      (Transformation|AddLocalOffset (Variables|Default|GetBox) (Math|Vector|MakeVector _range 0.0 0.0) false false)
      (Components|Box|SetBoxExtent (Variables|Default|GetBox) (Math|Vector|MakeVector _range (Variables|Default|GetWidthBoxDetection) (Variables|Default|GetHeightBoxDetection)) true))))

(event Game|Damage|EventAnyDamage
  (params (Damage :type Float%20%28single-precision%29) (DamageType :type Damage%20Type%20Object%20Reference) (InstigatedBy :type Controller%20Object%20Reference) (DamageCauser :type Actor%20Object%20Reference))
  ;[1 1 1] Taking Damage from Enemy
  (bind _output_get (Variables|Default|SetHealth (- (Variables|Default|GetHealth) Damage)))
  (if (<= _output_get 0.0)
    (Actor|DestroyActor)
    (Audio|PlaySound2D "/Game/Sound/SFX/CUE_TurretDestroy.CUE_TurretDestroy" 1.1 1.0 0.0 0 0)))

(fn ConstructionScript)

(fn AttackEnemy
  (bind _listofenemy1 (Variables|Default|GetListOfEnemy1))
  (bind _first (Variables|Default|GetFirst))
  (bind _second (Variables|Default|GetSecond))
  (bind _returnvalue (Transformation|GetWorldTransform _first))
  (bind _returnvalue_2 (Transformation|GetWorldTransform _second))
  (bind _output (Utilities|Array|Get(acopy) _listofenemy1))
  (Variables|/Game/Blueprints/Enemy/EnemySystemBP/BP_Enemyy.BP_Enemyy_C|SetHP _output (- (Variables|/Game/Blueprints/Enemy/EnemySystemBP/BP_Enemyy.BP_Enemyy_C|GetHP _output) (Variables|Default|GetDamage)))
  (Effects|SpawnEmitteratLocation "/Game/Muzzles/Particles/P_Muzzle56.P_Muzzle56" (.location _returnvalue) (.rotation _returnvalue))
  (Effects|SpawnEmitteratLocation "/Game/Muzzles/Particles/P_Muzzle56.P_Muzzle56" (.location _returnvalue_2) (.rotation _returnvalue_2))
  (Audio|SpawnSoundatLocation (Variables|Default|GetSFXShoot) (.location _returnvalue_2) "0, 0, 0" 1.0 1.0 (Variables|Default|GetSoundStart%20Time) (Variables|Default|GetAttenuation%20Settings) 0))