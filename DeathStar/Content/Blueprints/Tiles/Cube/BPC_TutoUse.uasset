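; Cube tile used in the turret step of the tutorial, active only while the game instance's Tuto flag is false.
; On BeginPlay its plane ignores Visibility traces and it binds to game instance dispatchers that re-enable touch blocking or blink Arrow1 three times as a hint.
; The first touch, after a short delay, disables the plane's blocking again and fires the TUTOTurretLink dispatcher.
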(event OnInputTouchBegin(Plane)
  (params (FingerIndex :type ETouchIndex%20Enum :default "Touch1") (TouchedComponent :type Primitive%20Component%20Object%20Reference))
  (Utilities|FlowControl|DoOnce false
    (:Completed
      (bind _asbp_game_instance (Utilities|Casting|CastToBP_GameInstance (Game|GetGameInstance)))
      (if (not (Variables|/Game/Blueprints/System/BP_GameInstance.BP_GameInstance_C|GetTuto _asbp_game_instance))
        (Utilities|FlowControl|Delay 0.5)
        (Collision|SetCollisionResponsetoChannel (Variables|Default|GetPlane) "ECC_Visibility" "ECR_Ignore")
        (Default|CallTUTOTurretLink _asbp_game_instance)))))

(event Custom|SetVisi
  (Collision|SetCollisionResponsetoChannel (Variables|Default|GetPlane) "ECC_Visibility" "ECR_Block"))

(event Custom|FlashPoint
  (bind _arrow1 (Variables|Default|GetArrow1))
  (bind _arrow1_2 (Variables|Default|GetArrow1))
  (bind _arrow1_3 (Variables|Default|GetArrow1))
  (Rendering|SetVisibility _arrow1_2 true false)
  (Utilities|FlowControl|Delay 1.0)
  (Rendering|SetVisibility _arrow1_2 false false)
  (Utilities|FlowControl|Delay 1.0)
  (Rendering|SetVisibility _arrow1_3 true false)
  (Utilities|FlowControl|Delay 1.0)
  (Rendering|SetVisibility _arrow1_3 false false)
  (Utilities|FlowControl|Delay 1.0)
  (Rendering|SetVisibility _arrow1 true false)
  (Utilities|FlowControl|Delay 1.0)
  (Rendering|SetVisibility _arrow1 false false))

(event EventBeginPlay
  (bind _returnvalue (Game|GetGameInstance))
  (bind _asbp_game_instance (Utilities|Casting|CastToBP_GameInstance _returnvalue))
  (if (not (Variables|/Game/Blueprints/System/BP_GameInstance.BP_GameInstance_C|GetTuto _asbp_game_instance))
    (Collision|SetCollisionResponsetoChannel (Variables|Default|GetPlane) "ECC_Visibility" "ECR_Ignore")
    (EventDispatchers|BindEventtoTUTOactivateTilesTurret _asbp_game_instance (delegate Custom|SetVisi))
    (EventDispatchers|BindEventtoTUTOFlashPointLight _asbp_game_instance (delegate Custom|FlashPoint))))

(fn ConstructionScript
  (|CallParentFunction))