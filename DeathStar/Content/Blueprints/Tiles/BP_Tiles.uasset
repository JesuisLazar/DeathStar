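; Buildable tile that the player taps to place a Laser, Plasma, Flak or Mortar turret.
; Selection toggles a material mask and the WBMainRef build buttons, which first-start tutorial state gates; Creation spawns and attaches the turret, then tints the tile by type.
; Damage drains shield, then armor-adjusted hitpoints seeded from BP_GameInstance, driving blink and color parameters until destruction.
; Tick rebinds the game instance's TurretSelected event, which deselects the tile.
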(event OnInputTouchEnd(Plane)
  (params (FingerIndex :type ETouchIndex%20Enum :default "Touch1") (TouchedComponent :type Primitive%20Component%20Object%20Reference))
  (bind _returnvalue (Game|GetGameInstance))
  (bind _asbp_game_instance (Utilities|Casting|CastToBP_GameInstance _returnvalue))
  ;[1 1 1 1 50] Selection Tile System
  ;;[1 1 1] When a tile is selected, call the Event if turret is already selected
  (Default|CallTileSelected _asbp_game_instance)
  (if (Variables|/Game/Blueprints/System/BP_GameInstance.BP_GameInstance_C|GetFirstStart _asbp_game_instance)
    ;;[1 1 1] Check if tuto is completed
    (if (Variables|/Game/Blueprints/System/BP_GameInstance.BP_GameInstance_C|GetGestureTutoCompleted _asbp_game_instance)
      ;;[1 1 1] Chek if is already selected
      (if (Variables|Default|GetSelected) :!label _label
        ;;[1 1 1] Deselect it
        (CallFunction|Deselect (Variables|/Game/Blueprints/System/BP_GameInstance.BP_GameInstance_C|GetSelectedTiles (.AsBP%20Game%20Instance (Utilities|Casting|CastToBP_GameInstance (Game|GetGameInstance)))))
        (else
          (Audio|PlaySound2D "/Game/Sound/SFX/CUE_TilesSelected.CUE_TilesSelected" 1.0 1.0 0.0 0 0)
          ;;[1 0.9996 0.9996] Deselect it if another tile is selected
          (CallFunction|Deselect (Variables|/Game/Blueprints/System/BP_GameInstance.BP_GameInstance_C|GetSelectedTiles (.AsBP%20Game%20Instance (Utilities|Casting|CastToBP_GameInstance (Game|GetGameInstance)))))
          ;;[1 1 1] Set himself as selected
          (Variables|Default|SetSelected true)
          (Rendering|Material|SetScalarParameterValueonMaterials (Variables|Default|GetPlane) "MaskSelection" 1.0)
          (Collision|SetCollisionEnabled (Variables|Default|GetPlane) "QueryAndPhysics")
          (CallFunction|DisplayConstructionMenu)
          ;;[1 0 0] Passer Game Mode
          (Variables|/Game/Blueprints/System/BP_GameInstance.BP_GameInstance_C|SetSelectedTiles (.AsBP%20Game%20Instance (Utilities|Casting|CastToBP_GameInstance (Game|GetGameInstance))) self))))
    (else
      (goto _label))))

(event Custom|Creation
  (bind _returnvalue (Game|Player|GetPlayerPawn 0))
  (bind _returnvalue_2 (Game|GetGameMode))
  (bind _arrow (Variables|Default|GetArrow))
  (bind _returnvalue_3 (Transformation|GetWorldTransform _arrow))
  (bind _asbp_game_mode (Utilities|Casting|CastToBP_GameMode _returnvalue_2))
  (bind _asbp_heart (Utilities|Casting|CastToBP_Heart _returnvalue))
  (bind _wbmainref (Variables|/Game/Blueprints/System/BP_Heart.BP_Heart_C|GetWBMainRef _asbp_heart))
  (bind _bt_newlaser (Variables|/Game/Blueprints/Widget/WB_Main.WB_Main_C|GetBT_NewLaser _wbmainref))
  (bind _bt_newflak (Variables|/Game/Blueprints/Widget/WB_Main.WB_Main_C|GetBT_NewFlak _wbmainref))
  (bind _widgetstyle (Variables|/Script/UMG.Button|GetWidgetStyle _bt_newflak))
  (bind _widgetstyle_2 (Variables|/Script/UMG.Button|GetWidgetStyle _bt_newlaser))
  (bind (_normal _hovered _pressed) (Utilities|Struct|BreakButtonStyle _widgetstyle_2))
  (bind (_normal_2 _hovered_2 _pressed_2) (Utilities|Struct|BreakButtonStyle _widgetstyle))
  ;[1 1 1 1 50] Creation Turret System
  (Variables|/Game/Blueprints/System/BP_GameInstance.BP_GameInstance_C|SetGestureTutoCompleted (.AsBP%20Game%20Instance (Utilities|Casting|CastToBP_GameInstance (Game|GetGameInstance))) true)
  (Math|Integer|IncrementInt (Variables|/Game/Blueprints/System/BP_GameMode.BP_GameMode_C|GetTurretCreated (.AsBP%20Game%20Mode (Utilities|Casting|CastToBP_GameMode (Game|GetGameMode))))
    (:%20%20
      ;;[1 1 1] Check if the tile is selected
      (if (Variables|Default|GetSelected)
        ;;[1 1 1] Spawn Turret on tile location
        (bind _returnvalue_4 (Game|SpawnActorfromClass (Variables|Default|GetActor) (Math|Transform|MakeTransform (.location _returnvalue_3) (.rotation _returnvalue_3) (Variables|Default|GetWeaponScale)) "Undefined" 0 0))
        ;;[1 1 1] Lock the turret to his tile
        (Transformation|AttachComponentToComponent _returnvalue_4 (Variables|Default|GetDefaultSceneRoot) "None" "KeepWorld" "KeepWorld" "SnapToTarget" true)
        (CallFunction|HidesConstructionMenu)
        ;;[1 1 1] A VOIR ENABLED DISABLED
        (Variables|Default|SetSelected false)
        (Collision|SetCollisionEnabled (Variables|Default|GetPlane) "QueryAndPhysics")
        (Rendering|Material|SetMaterial (Variables|Default|GetPlane) 0 (Variables|Default|GetMaterial))
        ;;[1 1 1] Apply color of the turret to the tile
        (if (== (Variables|Default|GetActor) "/Game/Blueprints/Defense/BPC_Laser.BPC_Laser_C")
          (Rendering|Material|SetVectorParameterValueonMaterials (Variables|Default|GetPlane) "TileColor" (Math|Conversions|ToVector(LinearColor) "(R=1.000000,G=0.000000,B=0.000000,A=1.000000)"))
          (Audio|SpawnSoundatLocation (Variables|Default|GetSoundConstruction) (.location (Transformation|GetWorldTransform (Variables|Default|GetArrow))) "0, 0, 0" 1.0 1.0 (Variables|Default|GetStart%20Time) (Variables|Default|GetAttenuation%20Settings) 0 :!label _label)
          ;;[1 1 1] Tuto
          (if (Variables|/Game/Blueprints/System/BP_GameInstance.BP_GameInstance_C|GetFirstStart (.AsBP%20Game%20Instance (Utilities|Casting|CastToBP_GameInstance (Game|GetGameInstance))))
            (if (== (Variables|/Game/Blueprints/System/BP_GameMode.BP_GameMode_C|GetTurretCreated _asbp_game_mode) 1)
              (Widget|SetVisibility (Variables|/Game/Blueprints/Widget/WB_Main.WB_Main_C|GetTxtIntro5 _wbmainref) "Visible")
              (Class|WidgetBlueprintLibrary|SetBrushResourcetoMaterial _normal "/Game/Blueprints/Widget/UI/LaserButton/M_LaserButton.M_LaserButton")
              (Class|WidgetBlueprintLibrary|SetBrushResourcetoMaterial _hovered "/Game/Blueprints/Widget/UI/LaserButton/M_LaserButton.M_LaserButton")
              (Class|WidgetBlueprintLibrary|SetBrushResourcetoMaterial _pressed "/Game/Blueprints/Widget/UI/LaserButton/M_LaserButton.M_LaserButton")
              (else
                (Default|CallTutoAfterWave2OK _asbp_game_mode)
                (Class|WidgetBlueprintLibrary|SetBrushResourcetoMaterial _normal_2 "/Game/Blueprints/Widget/UI/FlakButton/M_FlakButton.M_FlakButton")
                (Class|WidgetBlueprintLibrary|SetBrushResourcetoMaterial _hovered_2 "/Game/Blueprints/Widget/UI/FlakButton/M_FlakButton.M_FlakButton")
                (Class|WidgetBlueprintLibrary|SetBrushResourcetoMaterial _pressed_2 "/Game/Blueprints/Widget/UI/FlakButton/M_FlakButton.M_FlakButton"))))
          (elif (== (Variables|Default|GetActor) "/Game/Blueprints/Defense/BPC_Plasma.BPC_Plasma_C")
            (Rendering|Material|SetVectorParameterValueonMaterials (Variables|Default|GetPlane) "TileColor" (Math|Conversions|ToVector(LinearColor) "(R=0.008840,G=1.000000,B=0.000000,A=1.000000)"))
            (goto _label)
            (elif (== (Variables|Default|GetActor) "/Game/Blueprints/Defense/BPC_Flak.BPC_Flak_C")
              (Rendering|Material|SetVectorParameterValueonMaterials (Variables|Default|GetPlane) "TileColor" (Math|Conversions|ToVector(LinearColor) "(R=0.001875,G=0.000000,B=1.000000,A=1.000000)"))
              (goto _label)
              (elif (== (Variables|Default|GetActor) "/Game/Blueprints/Defense/BPC_Mortar.BPC_Mortar_C")
                (Rendering|Material|SetVectorParameterValueonMaterials (Variables|Default|GetPlane) "TileColor" (Math|Conversions|ToVector(LinearColor) "(R=1.000000,G=0.438163,B=0.000000,A=1.000000)"))
                (goto _label)))))))))

(event Custom|Turret%20Selected
  ;[1 1 1 1 50] Selection Tile System
  ;;[1 1 1] Deselect the tile when a Turret is selected
  (CallFunction|Deselect))

(event Custom|Deselect
  ;[1 1 1 1 50] Selection Tile System
  (Variables|Default|SetSelected false)
  (Rendering|Material|SetScalarParameterValueonMaterials (Variables|Default|GetPlane) "MaskSelection" 0.0)
  (CallFunction|HidesConstructionMenu)
  ;;[1 0 0] Passer Game Mode
  (Variables|/Game/Blueprints/System/BP_GameInstance.BP_GameInstance_C|SetSelectedTiles (.AsBP%20Game%20Instance (Utilities|Casting|CastToBP_GameInstance (Game|GetGameInstance))) 0))

(event Game|Damage|EventAnyDamage
  (params (Damage :type Float%20%28single-precision%29) (DamageType :type Damage%20Type%20Object%20Reference) (InstigatedBy :type Controller%20Object%20Reference) (DamageCauser :type Actor%20Object%20Reference))
  (bind _plane (Variables|Default|GetPlane))
  ;[1 1 1 1 50] Damage Tile System
  (Utilities|FlowControl|Sequence
    (:then_0
      (if (< (- (Variables|Default|GettilesCurrentShield) Damage) 0.0)
        (Variables|Default|SettilesCurrentHitpoints (- (Math|Float|Clamp(Float) (+ (Variables|Default|GettilesCurrentHitpoints) (- (Variables|Default|GettilesCurrentShield) Damage)) 0.0 (Variables|Default|GettilesMaxHitpoints)) (Variables|Default|GettilesArmor))))
      (Variables|Default|SettilesCurrentShield (Math|Float|Clamp(Float) (- (Variables|Default|GettilesCurrentShield) Damage) 0.0 (Variables|Default|GettilesMaxShield)))
      (if (<= (Variables|Default|GettilesCurrentHitpoints) 0.0)
        (Actor|DestroyActor)))
    (:then_1
      ;[1 1 1] Visual Feedback + Blinking
      (if (<= (Variables|Default|GettilesCurrentHitpoints) 3e+02)
        (Variables|FX|SetblinkingSpeed 0.0)
        (Variables|FX|SetColorLight (Variables|FX|GetfullLifeColor))))
    (:then_2
      (if (<= (Variables|Default|GettilesCurrentHitpoints) 2e+02)
        (Variables|FX|SetblinkingSpeed 2.0)
        (Variables|FX|SetColorLight (Variables|FX|GetmidLifeColor))))
    (:then_3
      (if (<= (Variables|Default|GettilesCurrentHitpoints) 1e+02)
        (Variables|FX|SetblinkingSpeed 4.0)
        (Variables|FX|SetColorLight (Variables|FX|GetlowLifeColor))))
    (:then_4
      (Rendering|Material|SetScalarParameterValueonMaterials _plane "NumberHit" (Variables|FX|GetblinkingSpeed))
      (Rendering|Material|SetVectorParameterValueonMaterials _plane "ColorLight" (Math|Vector|MakeVector (Math|Conversions|ToFloat(Byte) (.R (Math|Color|BreakColor (Variables|FX|GetColorLight)))) (Math|Conversions|ToFloat(Byte) (.G (Math|Color|BreakColor (Variables|FX|GetColorLight)))) (Math|Conversions|ToFloat(Byte) (.B (Math|Color|BreakColor (Variables|FX|GetColorLight)))))))))

(event EventTick
  (params (DeltaSeconds :type Float%20%28single-precision%29))
  ;[1 1 1 1 50] Selection Tile System
  ;;[1 1 1] Deselect the tile when a Turret is selected
  (EventDispatchers|BindEventtoTurretSelected (.AsBP%20Game%20Instance (Utilities|Casting|CastToBP_GameInstance (Game|GetGameInstance))) (delegate Custom|Turret%20Selected)))

(event EventBeginPlay
  ;[1 1 1] Set Value
  (CallFunction|SetGameInstanceValue))

(fn ConstructionScript)

(fn DisplayConstructionMenu
  (bind _returnvalue (Game|GetGameInstance))
  (bind _returnvalue_2 (Game|Player|GetPlayerPawn 0))
  (bind _returnvalue_3 (Game|GetGameInstance))
  (bind _returnvalue_4 (Game|Player|GetPlayerPawn 0))
  (bind _returnvalue_5 (Game|Player|GetPlayerPawn 0))
  (bind _asbp_game_instance (Utilities|Casting|CastToBP_GameInstance _returnvalue_3))
  (bind _asbp_heart (Utilities|Casting|CastToBP_Heart _returnvalue_2))
  (bind _asbp_game_instance_2 (Utilities|Casting|CastToBP_GameInstance _returnvalue))
  (bind _asbp_heart_2 (Utilities|Casting|CastToBP_Heart _returnvalue_5))
  (bind _asbp_heart_3 (Utilities|Casting|CastToBP_Heart _returnvalue_4))
  (bind _wbmainref (Variables|/Game/Blueprints/System/BP_Heart.BP_Heart_C|GetWBMainRef _asbp_heart_2))
  (bind _wbmainref_2 (Variables|/Game/Blueprints/System/BP_Heart.BP_Heart_C|GetWBMainRef _asbp_heart))
  (bind _waves (Variables|/Game/Blueprints/System/BP_GameInstance.BP_GameInstance_C|GetWaves _asbp_game_instance))
  (bind _wbmainref_3 (Variables|/Game/Blueprints/System/BP_Heart.BP_Heart_C|GetWBMainRef _asbp_heart_3))
  (bind _bt_newflak (Variables|/Game/Blueprints/Widget/WB_Main.WB_Main_C|GetBT_NewFlak _wbmainref_3))
  (bind _bt_newlaser (Variables|/Game/Blueprints/Widget/WB_Main.WB_Main_C|GetBT_NewLaser _wbmainref_2))
  (bind _widgetstyle (Variables|/Script/UMG.Button|GetWidgetStyle _bt_newflak))
  (bind _widgetstyle_2 (Variables|/Script/UMG.Button|GetWidgetStyle _bt_newlaser))
  (bind (_normal _hovered _pressed) (Utilities|Struct|BreakButtonStyle _widgetstyle))
  (bind (_normal_2 _hovered_2 _pressed_2) (Utilities|Struct|BreakButtonStyle _widgetstyle_2))
  (if (Variables|/Game/Blueprints/System/BP_GameInstance.BP_GameInstance_C|GetFirstStart (.AsBP%20Game%20Instance (Utilities|Casting|CastToBP_GameInstance (Game|GetGameInstance))))
    (if (< _waves 2)
      ;[1 1 1] Tuto
      (Widget|SetVisibility (Variables|/Game/Blueprints/Widget/WB_Main.WB_Main_C|GetBT_NewLaser _wbmainref) "Visible") ; affiche laser button
      (if (not (Variables|/Game/Blueprints/System/BP_GameInstance.BP_GameInstance_C|GetFirstTurretBuild _asbp_game_instance_2))
        (Variables|/Game/Blueprints/System/BP_GameInstance.BP_GameInstance_C|SetGestureTutoCompleted _asbp_game_instance_2 false) ; disable tile selection for first construction
        ;;[1 1 1] Affiche le text et fait clignoté le laser button
        (Widget|SetVisibility (Variables|/Game/Blueprints/Widget/WB_Main.WB_Main_C|GetTxtIntro2 _wbmainref) "Hidden")
        (Widget|SetVisibility (Variables|/Game/Blueprints/Widget/WB_Main.WB_Main_C|GetTxtIntro4 _wbmainref) "Visible")
        (Variables|/Game/Blueprints/System/BP_GameInstance.BP_GameInstance_C|SetFirstTurretBuild _asbp_game_instance_2 true)
        (Class|WidgetBlueprintLibrary|SetBrushResourcetoMaterial _normal_2 "/Game/Blueprints/Widget/UI/LaserButton/M_LaserTuto.M_LaserTuto")
        (Class|WidgetBlueprintLibrary|SetBrushResourcetoMaterial _hovered_2 "/Game/Blueprints/Widget/UI/LaserButton/M_LaserTuto.M_LaserTuto")
        (Class|WidgetBlueprintLibrary|SetBrushResourcetoMaterial _pressed_2 "/Game/Blueprints/Widget/UI/LaserButton/M_LaserTuto.M_LaserTuto"))
      (else
        ;;[1 1 1 1 30] tuto Wave 3 construction flak
        (if (== _waves 3)
          ;;;[1 1 1] Affiche le flak boutton et le fait clignoté
          (Widget|SetVisibility (Variables|/Game/Blueprints/Widget/WB_Main.WB_Main_C|GetBT_NewFlak _wbmainref_3) "Visible")
          (Class|WidgetBlueprintLibrary|SetBrushResourcetoMaterial _normal "/Game/Blueprints/Widget/UI/FlakButton/M_FlakTuto.M_FlakTuto")
          (Class|WidgetBlueprintLibrary|SetBrushResourcetoMaterial _hovered "/Game/Blueprints/Widget/UI/FlakButton/M_FlakTuto.M_FlakTuto")
          (Class|WidgetBlueprintLibrary|SetBrushResourcetoMaterial _pressed "/Game/Blueprints/Widget/UI/FlakButton/M_FlakTuto.M_FlakTuto"))))
    (else
      (Widget|SetVisibility (Variables|/Game/Blueprints/Widget/WB_Main.WB_Main_C|GetBT_NewLaser (Variables|/Game/Blueprints/System/BP_Heart.BP_Heart_C|GetWBMainRef (.AsBP%20Heart (Utilities|Casting|CastToBP_Heart (Game|Player|GetPlayerPawn 0))))) "Visible"))))

(fn HidesConstructionMenu
  (Widget|SetVisibility (Variables|/Game/Blueprints/Widget/WB_Main.WB_Main_C|GetBT_NewLaser (Variables|/Game/Blueprints/System/BP_Heart.BP_Heart_C|GetWBMainRef (.AsBP%20Heart (Utilities|Casting|CastToBP_Heart (Game|Player|GetPlayerPawn 0))))) "Hidden"))

(fn SetGameInstanceValue
  (bind _returnvalue (Game|GetGameInstance))
  (bind _asbp_game_instance (Utilities|Casting|CastToBP_GameInstance _returnvalue))
  (Variables|Default|SettilesCurrentHitpoints (Variables|/Game/Blueprints/System/BP_GameInstance.BP_GameInstance_C|GettilesGlobalCurrentHitpoints _asbp_game_instance))
  (Variables|Default|SettilesMaxHitpoints (Variables|/Game/Blueprints/System/BP_GameInstance.BP_GameInstance_C|GettilesGlobalMaxHitpoints _asbp_game_instance))
  (Variables|Default|SettilesArmor (Variables|/Game/Blueprints/System/BP_GameInstance.BP_GameInstance_C|GettilesArmorGlobalValue _asbp_game_instance)))