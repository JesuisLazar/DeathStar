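; Tutorial resource pickup that spins every tick and waits to be collected by a screen touch.
; Its Box ignores queries until a short delay after BeginPlay, then becomes touchable.
; On touch release it has BP_GameMode award enemy-destruction materials, plays a pickup sound and hides the Collectible widget through the BP_Heart pawn's main widget.
; It then tells the game mode to continue the tutorial and destroys itself.
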(event OnInputTouchEnd(Box)
  (params (FingerIndex :type ETouchIndex%20Enum :default "Touch1") (TouchedComponent :type Primitive%20Component%20Object%20Reference))
  ;[1 1 1] Add Ressource to the player when it touch it
  (bind _asbp_game_mode (Utilities|Casting|CastToBP_GameMode (Game|GetGameMode)))
  (Default|AddMaterialsforEnemyDestruction _asbp_game_mode)
  (Audio|PlaySound2D "/Game/Sound/EnemySFX/RessourcePickUp.RessourcePickUp" 1.0 1.0 0.0 0 0)
  (Widget|SetVisibility (Variables|/Game/Blueprints/Widget/WB_Main.WB_Main_C|GetCollectible (Variables|/Game/Blueprints/System/BP_Heart.BP_Heart_C|GetWBMainRef (.AsBP%20Heart (Utilities|Casting|CastToBP_Heart (Game|Player|GetPlayerPawn 0))))) "Hidden")
  (Default|CallTutoAfterCollectible _asbp_game_mode)
  (Actor|DestroyActor))

(event EventBeginPlay
  ;[1 1 1] Destroy Ressource after 2sec if player don't touch it
  (Collision|SetCollisionEnabled (Variables|Default|GetBox) "NoCollision")
  (Utilities|FlowControl|Delay 3.0)
  (Collision|SetCollisionEnabled (Variables|Default|GetBox) "QueryOnly"))

(event EventTick
  (params (DeltaSeconds :type Float%20%28single-precision%29))
  (Transformation|AddActorLocalRotation "1.000000,1.000000,1.000000" false false))

(fn ConstructionScript)