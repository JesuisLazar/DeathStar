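; BP_Enemyy is a floating enemy that follows the player and fires hitscan attacks.
; On BeginPlay it hands detection points to FloatingAIMovement, which moves it each Tick, and starts an endless delayed loop of ammo-sized volleys separated by reload pauses.
; Each Attack line-traces forward from the Arrow, with debug drawing, and applies damage to the hit actor.
; Tick destroys it at zero Health; a health-based material change is left unconnected.
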(event EventBeginPlay
  (Utilities|FlowControl|Sequence
    (:then_0
      (Default|Setup (Variables|Default|GetFloating_AI_Movement) self (Game|Player|GetPlayerPawn 0) 0 (Variables|Default|GetFloating_AI_Behind_Detection_Location) (Variables|Default|GetFloating_AI_Behind_Up_Detection_Location) (Variables|Default|GetFloating_AI_Behind_Down_Detection_Location) (Variables|Default|GetFloating_AI_Right_Detection_Location) (Variables|Default|GetFloating_AI_Right_Up_Detection_Location) (Variables|Default|GetFloating_AI_Right_Down_Detection_Location) (Variables|Default|GetFloating_AI_Left_Detection_Location) (Variables|Default|GetFloating_AI_Left_Up_Detection_Location) (Variables|Default|GetFloating_AI_Left_Down_Detection_Location) (Variables|Default|GetFloating_AI_Middle_Of_Mesh_Location)))
    (:then_1
      (Utilities|ForLoopwithDelay 0 (- (Variables|Default|GetNbOfAmmo) 1) 1.0 :!label _label
        (:Loop%20Body
          (CallFunction|Attack))
        (:Completed
          (Utilities|FlowControl|Delay (Variables|Default|GetReloadDuration))
          (Variables|Default|SetNbOfAmmo (Variables|Default|GetNbOfAmmo))
          (goto _label))))))

(event EventTick
  (params (DeltaSeconds :type Float%20%28single-precision%29))
  (Default|Move (Variables|Default|GetFloating_AI_Movement))
  (Utilities|FlowControl|Sequence
    (:then_1
      ;[1 1 1] mort
      (if (<= (Variables|Default|GetHealth) 0.0)
        (Actor|DestroyActor)))))

(fn ConstructionScript)

(fn Attack
  (bind _arrow (Variables|Default|GetArrow))
  (bind _returnvalue (Transformation|GetWorldLocation _arrow))
  (bind _outhit (Collision|LineTraceByChannel _returnvalue (+ _returnvalue (* (Math|Vector|GetForwardVector _arrow) 2e+03)) "TraceTypeQuery1" false 0 "ForDuration" true "(R=1.000000,G=0.000000,B=0.000000,A=1.000000)" "(R=0.000000,G=1.000000,B=0.000000,A=1.000000)" 1e+01))
  (Game|Damage|ApplyDamage (.HitActor (Collision|BreakHitResult _outhit)) (Variables|Default|GetBase%20Damage) 0 0))