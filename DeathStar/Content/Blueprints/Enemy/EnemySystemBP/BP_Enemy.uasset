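; Wave enemy for a turret defense game that moves via FloatingAIMovement and line-trace attacks turrets, tiles and the Heart in timed bursts.
; Damage passes through shield and armor, with Flak and Plasma upgrade bypasses; mortar events temporarily slow it.
; Death may drop resources, awards materials and decrements its wave's GameMode counter.
; Flak, Plasma and suicide-Martyr behaviors key off world-wide GetActorOfClass lookups, not the damage causer or self.
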(event Custom|EnemyTakingDamage
  (bind _ph_shield (Variables|Default|GetPH_Shield))
  ;[1 1 1] TakingDamageFeedback
  (Rendering|SetVisibility _ph_shield true false)
  (Utilities|FlowControl|Delay 0.1)
  (Rendering|SetVisibility _ph_shield false false))

(event Custom|gettingSlowedByMortar
  (bind _floating_ai_movement (Variables|Default|GetFloating_AI_Movement))
  (bind _floating_ai_movement_2 (Variables|Default|GetFloating_AI_Movement))
  ;[1 1 1] Mortar Has Slowing Upgrade
  (Default|SetMoveSpeed _floating_ai_movement_2 (* (Variables|/Game/Blueprints/System/FloatingAIMovement/Blueprints/Floating_AI_Movement.Floating_AI_Movement_C|GetMoveSpeed _floating_ai_movement_2) 0.5))
  (Utilities|FlowControl|RetriggerableDelay 3.0)
  (Default|SetMoveSpeed _floating_ai_movement (* (Variables|/Game/Blueprints/System/FloatingAIMovement/Blueprints/Floating_AI_Movement.Floating_AI_Movement_C|GetMoveSpeed _floating_ai_movement) 1.5))
  (Development|PrintString "CUSTOMEVENTCALLEDSLOOOOW" true true "(R=1.000000,G=0.000000,B=0.000000,A=1.000000)"))

(event EventBeginPlay
  (EventDispatchers|BindEventtoGettingSlowedbyMortar (.AsBP%20Game%20Mode (Utilities|Casting|CastToBP_GameMode (Game|GetGameMode))) (delegate Custom|gettingSlowedByMortar))
  ;[1 1 1] Assigne la wave acutelle à l'enemy
  (Variables|Default|SetNbWave (Variables|/Game/Blueprints/System/BP_GameInstance.BP_GameInstance_C|GetWaves (.AsBP%20Game%20Instance (Utilities|Casting|CastToBP_GameInstance (Game|GetGameInstance)))))
  ;[1 1 1] Set the UI life of enemy
  (bind _asui_life_enemy (Utilities|Casting|CastToUI_LifeEnemy (UserInterface|GetUserWidgetObject (Variables|Default|GetWidget))))
  (Variables|/Game/Blueprints/Widget/UI_LifeEnemy.UI_LifeEnemy_C|SetActor _asui_life_enemy self)
  ;[1 1 1] Set the price of Enemy in the game mode
  (Variables|/Game/Blueprints/System/BP_GameMode.BP_GameMode_C|SetEnemyPrice (.AsBP%20Game%20Mode (Utilities|Casting|CastToBP_GameMode (Game|GetGameMode))) (Variables|Default|GetEnemyPrice))
  (Utilities|FlowControl|Sequence
    (:then_0
      (bind _floating_ai_movement (CallFunction|SetupFloating)))
    (:then_1
      (Default|SetMoveSpeed _floating_ai_movement (Variables|Default|GetMovementSpeed)))
    (:then_2
      ;[1 1 1] Attack System
      (Utilities|ForLoopwithDelay 0 (- (Variables|Default|GetNbOfAmmo) 1) (Variables|Default|GetDelayBtwAtk) :!label _label
        (:Loop%20Body
          (CallFunction|Attack))
        (:Completed
          (Utilities|FlowControl|Delay (Variables|Default|GetReloadDuration))
          (Variables|Default|SetNbOfAmmo (Variables|Default|GetNbOfAmmo))
          (goto _label))))
    (:then_3
      ;[1 1 1] Shield System
      (if (> (Variables|Default|GetmaxShield) 1.0)
        (Variables|Default|SethasShield true)))
    (:then_4
      ;[1 1 1] Armor System
      (if (> (Variables|Default|Getarmor) 1.0)
        (Variables|Default|SethasArmor true)))))

(event Game|Damage|EventAnyDamage
  (params (Damage :type Float%20%28single-precision%29) (DamageType :type Damage%20Type%20Object%20Reference) (InstigatedBy :type Controller%20Object%20Reference) (DamageCauser :type Actor%20Object%20Reference))
  (bind _returnvalue (Game|GetGameInstance))
  (bind _asbp_game_instance (Utilities|Casting|CastToBP_GameInstance _returnvalue))
  (if (Variables|Default|GethasShield)
    (bind _returnvalue_2 (Actor|GetActorOfClass "/Game/Blueprints/Defense/BPC_Flak.BPC_Flak_C"))
    (if (and (== (Utilities|GetClass _returnvalue_2) "/Game/Blueprints/Defense/BPC_Flak.BPC_Flak_C") (Variables|/Game/Blueprints/System/BP_GameInstance.BP_GameInstance_C|GetflakHasIgnoreShieldUpgrade _asbp_game_instance))
      (if (Variables|Default|GethasArmor) :!label _label
        (bind _returnvalue_3 (Actor|GetActorOfClass "/Game/Blueprints/Defense/BPC_Plasma.BPC_Plasma_C"))
        (if (and (== (Utilities|GetClass _returnvalue_3) "/Game/Blueprints/Defense/BPC_Plasma.BPC_Plasma_C") (Variables|/Game/Blueprints/System/BP_GameInstance.BP_GameInstance_C|GetplasmaHasIgnoreArmorUpgrade _asbp_game_instance))
          (Variables|Default|SetHP (- (Variables|Default|GetHP) Damage) :!label _label_2)
          (else
            ;[1 1 1] Enemy has Armor
            (if (Variables|Default|GethasArmor)
              (Variables|Default|SetHP (- (Variables|Default|GetHP) (- Damage (Variables|Default|Getarmor)))))))
        (else
          (goto _label_2)))
      (else
        ;[1 1 1] Enemy has Shield
        (if (< (- (Variables|Default|GetcurrentShield) Damage) 0.0)
          (Variables|Default|SetHP (Math|Float|Clamp(Float) (+ (Variables|Default|GetHP) (- (Variables|Default|GetcurrentShield) Damage)) 0.0 (Variables|Default|GetMaxHP))))
        (Variables|Default|SetcurrentShield (Math|Float|Clamp(Float) (- (Variables|Default|GetcurrentShield) Damage) 0.0 (Variables|Default|GetMaxHP)))))
    (else
      (goto _label))))

(event EventTick
  (params (DeltaSeconds :type Float%20%28single-precision%29))
  (bind _returnvalue (Game|GetGameMode))
  (bind _asbp_game_mode (Utilities|Casting|CastToBP_GameMode _returnvalue))
  (Default|Move (stale EventBeginPlay _floating_ai_movement))
  (bind _returnvalue_2 (Actor|GetActorOfClass "/Game/Blueprints/Enemy/BPC_Martyr.BPC_Martyr_C"))
  (if (== (Utilities|GetClass _returnvalue_2) "/Game/Blueprints/Enemy/BPC_Martyr.BPC_Martyr_C")
    (Default|OverrideMovetoLocation (Variables|Default|GetFloating_AI_Movement) "0, 0, 0" false -1.0))
  ;[1 1 1] If HP = 0
  (if (<= (Variables|Default|GetHP) 0.0)
    ;[1 1 1] Spawn Resources Once time on 5 at the position where the enemy dies
    (if (!= (Math|Random|RandomIntegerinRange 0 5) 1)
      _
      (else
        (Game|SpawnActorfromClass "/Game/Blueprints/Enemy/BP_Resources.BP_Resources_C" (Transformation|GetWorldTransform (Variables|Default|GetDefaultSceneRoot)) "Undefined" 0 0)))
    (Actor|DestroyActor)
    (Default|AddMaterialsforEnemyDestruction _asbp_game_mode)
    ;[1 1 1] Si l'ennemi détruit fait partie de la Wave 1, il retiré 1 au total d'ennemy alive de la wave 1
    (if (== (Variables|Default|GetNbWave) 1)
      (Math|Integer|DecrementInt (Variables|/Game/Blueprints/System/BP_GameMode.BP_GameMode_C|GetW1EnemyAlive _asbp_game_mode))
      (else
        ;[1 1 1] Si l'ennemi détruit fait partie de la Wave 2, il retiré 1 au total d'ennemy alive de la wave 2
        (if (== (Variables|Default|GetNbWave) 2)
          (Math|Integer|DecrementInt (Variables|/Game/Blueprints/System/BP_GameMode.BP_GameMode_C|GetW2EnemyAlive _asbp_game_mode))
          (else
            ;[1 1 1] Si l'ennemi détruit fait partie de la Wave 1, il retiré 1 au total d'ennemy alive de la wave 1
            (if (== (Variables|Default|GetNbWave) 3)
              (Math|Integer|DecrementInt (Variables|/Game/Blueprints/System/BP_GameMode.BP_GameMode_C|GetW3EnemyAlive _asbp_game_mode))
              (else
                ;[1 1 1] Si l'ennemi détruit fait partie de la Wave 1, il retiré 1 au total d'ennemy alive de la wave 1
                (if (== (Variables|Default|GetNbWave) 4)
                  (Math|Integer|DecrementInt (Variables|/Game/Blueprints/System/BP_GameMode.BP_GameMode_C|GetW4EnemyAlive _asbp_game_mode))
                  (else
                    ;[1 1 1] Si l'ennemi détruit fait partie de la Wave 1, il retiré 1 au total d'ennemy alive de la wave 1
                    (if (== (Variables|Default|GetNbWave) 5)
                      (Math|Integer|DecrementInt (Variables|/Game/Blueprints/System/BP_GameMode.BP_GameMode_C|GetW5EnemyAlive _asbp_game_mode))
                      (else
                        ;[1 1 1] Si l'ennemi détruit fait partie de la Wave 1, il retiré 1 au total d'ennemy alive de la wave 1
                        (if (== (Variables|Default|GetNbWave) 6)
                          (Math|Integer|DecrementInt (Variables|/Game/Blueprints/System/BP_GameMode.BP_GameMode_C|GetW6EnemyAlive _asbp_game_mode))
                          (else
                            ;[1 1 1] Si l'ennemi détruit fait partie de la Wave 1, il retiré 1 au total d'ennemy alive de la wave 1
                            (if (== (Variables|Default|GetNbWave) 7)
                              (Math|Integer|DecrementInt (Variables|/Game/Blueprints/System/BP_GameMode.BP_GameMode_C|GetW7EnemyAlive _asbp_game_mode))
                              (else
                                ;[1 1 1] Si l'ennemi détruit fait partie de la Wave 1, il retiré 1 au total d'ennemy alive de la wave 1
                                (if (== (Variables|Default|GetNbWave) 8)
                                  (Math|Integer|DecrementInt (Variables|/Game/Blueprints/System/BP_GameMode.BP_GameMode_C|GetW8EnemyAlive _asbp_game_mode))
                                  (else
                                    ;[1 1 1] Si l'ennemi détruit fait partie de la Wave 1, il retiré 1 au total d'ennemy alive de la wave 1
                                    (if (== (Variables|Default|GetNbWave) 9)
                                      (Math|Integer|DecrementInt (Variables|/Game/Blueprints/System/BP_GameMode.BP_GameMode_C|GetW9EnemyAlive _asbp_game_mode))
                                      (else
                                        ;[1 1 1] Si l'ennemi détruit fait partie de la Wave 1, il retiré 1 au total d'ennemy alive de la wave 1
                                        (if (== (Variables|Default|GetNbWave) 10)
                                          (Math|Integer|DecrementInt (Variables|/Game/Blueprints/System/BP_GameMode.BP_GameMode_C|GetW10EnemyAlive _asbp_game_mode)))))))))))))))))))))))

(fn ConstructionScript)

(fn Attack
  (bind _first (Variables|Default|GetFirst))
  (bind _arrow (Variables|Default|GetArrow))
  (bind _second (Variables|Default|GetSecond))
  (bind _emitter_template (Variables|Default|GetEmitter%20Template))
  (bind _returnvalue (Transformation|GetWorldLocation _arrow))
  (bind _returnvalue_2 (Transformation|GetWorldTransform _first))
  (bind _returnvalue_3 (Transformation|GetWorldTransform _second))
  (bind _outhit (Collision|LineTraceByChannel _returnvalue (+ _returnvalue (* (Math|Vector|GetForwardVector _arrow) (Variables|Default|GetRange))) "TraceTypeQuery1" false 0 "ForDuration"))
  (if (Math|Boolean|ORBoolean (Utilities|ClassIsChildOf (Utilities|GetClass (.HitActor (Collision|BreakHitResult _outhit))) "/Game/Blueprints/Defense/DefenseSystemBP/BP_Turret.BP_Turret_C") (Utilities|ClassIsChildOf (Utilities|GetClass (.HitActor (Collision|BreakHitResult _outhit))) "/Game/Blueprints/Tiles/Cube/BP_Tiles.BP_Tiles_C") (== (Utilities|GetClass (.HitActor (Collision|BreakHitResult _outhit))) "/Game/Blueprints/System/BP_Heart.BP_Heart_C") (== (Utilities|GetClass (.HitActor (Collision|BreakHitResult _outhit))) "/Game/Blueprints/Tiles/Cube/BP_frame_Blueprint.BP_frame_Blueprint_C"))
    (Game|Damage|ApplyDamage (.HitActor (Collision|BreakHitResult _outhit)) (Variables|Default|GetDamage) 0 self)
    (bind _returnvalue_4 (Actor|GetActorOfClass "/Game/Blueprints/Enemy/BPC_Martyr.BPC_Martyr_C"))
    (if (== (Utilities|GetClass _returnvalue_4) "/Game/Blueprints/Enemy/BPC_Martyr.BPC_Martyr_C")
      (Actor|DestroyActor)
      (else
        (Effects|SpawnEmitteratLocation _emitter_template (.location _returnvalue_2) (.rotation _returnvalue_2) (.scale _returnvalue_2))
        (Effects|SpawnEmitteratLocation _emitter_template (.location _returnvalue_3) (.rotation _returnvalue_3) (.scale _returnvalue_3))
        (Audio|SpawnSoundatLocation (Variables|Default|GetSFXShoot) (.location _returnvalue_3) "0, 0, 0" (Variables|Default|GetVolume%20Multiplier) 1.0 (Variables|Default|GetSoundStart%20Time) (Variables|Default|GetAttenuation%20Settings) 0)))))

(fn SetupFloating
  (bind _floating_ai_movement (Variables|Default|GetFloating_AI_Movement))
  (Default|Setup _floating_ai_movement self (Game|Player|GetPlayerPawn 0) 0 (Variables|Default|GetFloating_AI_Behind_Detection_Location) (Variables|Default|GetFloating_AI_Behind_Up_Detection_Location) (Variables|Default|GetFloating_AI_Behind_Down_Detection_Location) (Variables|Default|GetFloating_AI_Right_Detection_Location) (Variables|Default|GetFloating_AI_Right_Up_Detection_Location) (Variables|Default|GetFloating_AI_Right_Down_Detection_Location) (Variables|Default|GetFloating_AI_Left_Detection_Location) (Variables|Default|GetFloating_AI_Left_Up_Detection_Location) (Variables|Default|GetFloating_AI_Left_Down_Detection_Location) (Variables|Default|GetFloating_AI_Middle_Of_Mesh_Location))
  (return _floating_ai_movement))