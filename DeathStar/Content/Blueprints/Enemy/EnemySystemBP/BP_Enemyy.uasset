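; Flying enemy actor that pursues the player pawn, fires hitscan attacks and awards gold on death.
; BeginPlay stores its price in the GameInstance, sets up a FloatingAIMovement with directional detection points, and Tick drives that movement.
; An endless delayed loop fires a burst of forward Visibility line traces from the Arrow, applying damage, then waits to reload.
; Tick also polls HP, destroying the actor and calling the GameMode's AddGold at zero.
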(event EventBeginPlay
  (Variables|/Game/Blueprints/System/BP_GameInstance.BP_GameInstance_C|SetEnemyPrice (.AsBP%20Game%20Instance (Utilities|Casting|CastToBP_GameInstance (Game|GetGameInstance))) (Variables|Default|GetEnemyPrice))
  (Utilities|FlowControl|Sequence
    (:then_0
      (bind _floating_ai_movement (CallFunction|SetupFloating)))
    (:then_1
      (Utilities|ForLoopwithDelay 0 (- (Variables|Default|GetNbOfAmmo) 1) (Variables|Default|GetDelayBtwAtk) :!label _label
        (:Loop%20Body
          (CallFunction|Attack))
        (:Completed
          (Utilities|FlowControl|Delay (Variables|Default|GetReloadDuration))
          (Variables|Default|SetNbOfAmmo (Variables|Default|GetNbOfAmmo))
          (goto _label))))
    (:then_2
      (Default|SetMoveSpeed _floating_ai_movement (Variables|Default|GetMovementSpeed)))))

(event EventTick
  (params (DeltaSeconds :type Float%20%28single-precision%29))
  (Default|Move (stale EventBeginPlay _floating_ai_movement))
  ;[1 1 1] Death (Checking with event dispatch for game ressource)
  (if (<= (Variables|Default|GetHP) 0.0)
    (Actor|DestroyActor)
    (Default|AddGold (.AsBP%20Game%20Mode (Utilities|Casting|CastToBP_GameMode (Game|GetGameMode))))))

(fn ConstructionScript)

(fn Attack
  (bind _arrow (Variables|Default|GetArrow))
  (bind _returnvalue (Transformation|GetWorldLocation _arrow))
  (bind _outhit (Collision|LineTraceByChannel _returnvalue (+ _returnvalue (* (Math|Vector|GetForwardVector _arrow) (Variables|Default|GetRange))) "TraceTypeQuery1" false 0 "None"))
  (Game|Damage|ApplyDamage (.HitActor (Collision|BreakHitResult _outhit)) (Variables|Default|GetDamage) 0 0))

(fn SetupFloating
  (bind _floating_ai_movement (Variables|Default|GetFloating_AI_Movement))
  (Default|Setup _floating_ai_movement self (Game|Player|GetPlayerPawn 0) 0 (Variables|Default|GetFloating_AI_Behind_Detection_Location) (Variables|Default|GetFloating_AI_Behind_Up_Detection_Location) (Variables|Default|GetFloating_AI_Behind_Down_Detection_Location) (Variables|Default|GetFloating_AI_Right_Detection_Location) (Variables|Default|GetFloating_AI_Right_Up_Detection_Location) (Variables|Default|GetFloating_AI_Right_Down_Detection_Location) (Variables|Default|GetFloating_AI_Left_Detection_Location) (Variables|Default|GetFloating_AI_Left_Up_Detection_Location) (Variables|Default|GetFloating_AI_Left_Down_Detection_Location) (Variables|Default|GetFloating_AI_Middle_Of_Mesh_Location))
  (return _floating_ai_movement))