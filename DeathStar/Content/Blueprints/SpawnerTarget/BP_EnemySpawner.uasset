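; Enemy spawner that releases up to four waves of enemies, each started by an event bound through BP_GameInstance.
; On BeginPlay it shows a laser particle if wave one has first-group enemies, and hides it when a wave event fires.
; Each wave waits, then runs two chained delayed loops, each spawning a configurable enemy type and count.
; Spawned enemies receive a FloatingAIMovement destination randomly offset around the Target's box.
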(event Custom|Laser
  (Rendering|SetVisibility (Variables|Default|GetParticleSystem) true false))

(event Custom|Waves2
  (bind _enemy1 (Variables|Default|GetEnemy1))
  (bind _enemy2 (Variables|Default|GetEnemy2))
  ;[1 1 1] Waves2
  (Rendering|SetVisibility (Variables|Default|GetParticleSystem) false false)
  (Utilities|FlowControl|Delay (Variables|Default|GetW2DelayOfTheWaves))
  (Utilities|ForLoopwithDelay 0 (- (Variables|Default|GetW2NumberOfEnemy1) 1) (Variables|Default|GetW2SpawnDelay1)
    (:Loop%20Body
      (CallFunction|Spawn (Utilities|Select :Index (Variables|Default|GetW2FirstEnemy1) :NewEnumerator0 _enemy1 :NewEnumerator1 _enemy2)))
    (:Completed
      (Utilities|ForLoopwithDelay 0 (- (Variables|Default|GetW2NumberOfEnemy2) 1) (Variables|Default|GetW2SpawnDelay2)
        (:Loop%20Body
          (CallFunction|Spawn (Utilities|Select :Index (Variables|Default|GetW2FirstEnemy2) :NewEnumerator0 _enemy1 :NewEnumerator1 _enemy2)))))))

(event Custom|StartWave
  (bind _enemy1 (Variables|Default|GetEnemy1))
  (bind _enemy2 (Variables|Default|GetEnemy2))
  ;[1 1 1] Waves1
  (Rendering|SetVisibility (Variables|Default|GetParticleSystem) false false)
  (Utilities|FlowControl|Delay (Variables|Default|GetW1DelayOfTheWaves))
  (Utilities|ForLoopwithDelay 0 (- (Variables|Default|GetW1NumberOfEnemy1) 1) (Variables|Default|GetW1SpawnDelay1)
    (:Loop%20Body
      (CallFunction|Spawn (Utilities|Select :Index (Variables|Default|GetW1FirstEnemy1) :NewEnumerator0 _enemy1 :NewEnumerator1 _enemy2)))
    (:Completed
      (Utilities|ForLoopwithDelay 0 (- (Variables|Default|GetW1NumberOfEnemy2) 1) (Variables|Default|GetW1SpawnDelay2)
        (:Loop%20Body
          (CallFunction|Spawn (Utilities|Select :Index (Variables|Default|GetW1SecondEnemy2) :NewEnumerator0 _enemy1 :NewEnumerator1 _enemy2)))))))

(event Custom|Waves3
  (bind _enemy1 (Variables|Default|GetEnemy1))
  (bind _enemy2 (Variables|Default|GetEnemy2))
  ;[1 1 1] Waves3
  (Rendering|SetVisibility (Variables|Default|GetParticleSystem) false false)
  (Utilities|FlowControl|Delay (Variables|Default|GetW3DelayOfTheWaves))
  (Utilities|ForLoopwithDelay 0 (- (Variables|Default|GetW3NumberOfEnemy1) 1) (Variables|Default|GetW3SpawnDelay1)
    (:Loop%20Body
      (CallFunction|Spawn (Utilities|Select :Index (Variables|Default|GetW3FirstEnemy1) :NewEnumerator0 _enemy1 :NewEnumerator1 _enemy2)))
    (:Completed
      (Utilities|ForLoopwithDelay 0 (- (Variables|Default|GetW3NumberOfEnemy2) 1) (Variables|Default|GetW3SpawnDelay2)
        (:Loop%20Body
          (CallFunction|Spawn (Utilities|Select :Index (Variables|Default|GetW3FirstEnemy2) :NewEnumerator0 _enemy1 :NewEnumerator1 _enemy2)))))))

(event Custom|Waves4
  (bind _enemy1 (Variables|Default|GetEnemy1))
  (bind _enemy2 (Variables|Default|GetEnemy2))
  ;[1 1 1] Waves4
  (Rendering|SetVisibility (Variables|Default|GetParticleSystem) false false)
  (Utilities|FlowControl|Delay (Variables|Default|GetW4DelayOfTheWaves))
  (Utilities|ForLoopwithDelay 0 (- (Variables|Default|GetW4NumberOfEnemy1) 1) (Variables|Default|GetW4SpawnDelay1)
    (:Loop%20Body
      (CallFunction|Spawn (Utilities|Select :Index (Variables|Default|GetW4FirstEnemy1) :NewEnumerator0 _enemy1 :NewEnumerator1 _enemy2)))
    (:Completed
      (Utilities|ForLoopwithDelay 0 (- (Variables|Default|GetW4NumberOfEnemy2) 1) (Variables|Default|GetW4SpawnDelay2)
        (:Loop%20Body
          (CallFunction|Spawn (Utilities|Select :Index (Variables|Default|GetW4FirstEnemy2) :NewEnumerator0 _enemy1 :NewEnumerator1 _enemy2)))))))

(event EventBeginPlay
  (bind _returnvalue (Game|GetGameInstance))
  (bind _asbp_game_instance (Utilities|Casting|CastToBP_GameInstance _returnvalue))
  (if (> (Variables|Default|GetW1NumberOfEnemy1) 0)
    (CallFunction|Laser))
  (EventDispatchers|BindEventtoOnStart _asbp_game_instance (delegate Custom|StartWave))
  (EventDispatchers|BindEventtoWaves2 _asbp_game_instance (delegate Custom|Waves2))
  (EventDispatchers|BindEventtoWaves3 _asbp_game_instance (delegate Custom|Waves3))
  (EventDispatchers|BindEventtoWaves4 _asbp_game_instance (delegate Custom|Waves4)))

(fn ConstructionScript)

(fn Spawn
  (params (Enemy :type Actor%20Class%20Reference))
  (bind _returnvalue (Transformation|GetActorTransform))
  (bind _returnvalue_2 (Math|Random|RandomFloatinRange 1.0 1.0))
  (bind _asbp_enemyy (Utilities|Casting|CastToBP_EnemyyClass Enemy))
  (bind _returnvalue_3 (Game|SpawnActorfromClass _asbp_enemyy (Math|Transform|MakeTransform (.location _returnvalue) (.rotation _returnvalue) (Math|Vector|MakeVector _returnvalue_2 _returnvalue_2 _returnvalue_2)) "AlwaysSpawn" 0 0))
  (Default|OverrideMovetoLocation (Variables|/Game/Blueprints/Enemy/EnemySystemBP/BP_Enemyy.BP_Enemyy_C|GetFloating_AI_Movement _returnvalue_3) (+ (Transformation|GetWorldLocation (Variables|/Game/Blueprints/SpawnerTarget/BP_Target.BP_Target_C|GetBox (Variables|Default|GetTarget))) (* (Math|Vector|Normalize (Math|Random|RandomUnitVector)) 120)) true 0.0))