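; Skybox actor that shows an irregular galaxy backdrop built from six face meshes, one per axis direction, using the ESO34931 texture set.
; The construction script creates a dynamic material instance for each face and applies it to that face.
; It then assigns each face its matching texture and pushes a shared Brightness value to all six materials.
; The event graph holds no active logic.
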(event EventBeginPlay)

(event Collision|EventActorBeginOverlap
  (params (OtherActor :type Actor%20Object%20Reference)))

(event EventTick
  (params (DeltaSeconds :type Float%20%28single-precision%29)))

(fn ConstructionScript
  (CallFunction|CreateMaterials)
  (CallFunction|ApplyMaterials)
  (CallFunction|SetTextures))

(fn ApplyMaterials
  ;[1 1 1] Apply all created material instances to the corresponding sides
  (Rendering|Material|SetMaterial (Variables|Default|Getx_pos) 0 (Variables|Materials|GetXPosMat))
  (Rendering|Material|SetMaterial (Variables|Default|Getz_pos) 0 (Variables|Materials|GetZPosMat))
  (Rendering|Material|SetMaterial (Variables|Default|Getx_neg) 0 (Variables|Materials|GetXNegMat))
  (Rendering|Material|SetMaterial (Variables|Default|Getz_neg) 0 (Variables|Materials|GetZNegMat))
  (Rendering|Material|SetMaterial (Variables|Default|Gety_pos) 0 (Variables|Materials|GetYPosMat))
  (Rendering|Material|SetMaterial (Variables|Default|Gety_neg) 0 (Variables|Materials|GetYNegMat)))

(fn CreateMaterials
  ;[1 1 1] Create material instances to set the textures
  (bind _returnvalue (Rendering|Material|CreateDynamicMaterialInstance (Variables|Default|Getx_neg) 0 0 "None" :!class /Script/Engine.PrimitiveComponent))
  (Variables|Materials|SetXNegMat _returnvalue)
  (bind _returnvalue_2 (Rendering|Material|CreateDynamicMaterialInstance (Variables|Default|Getx_pos) 0 0 "None" :!class /Script/Engine.PrimitiveComponent))
  (Variables|Materials|SetXPosMat _returnvalue_2)
  (bind _returnvalue_3 (Rendering|Material|CreateDynamicMaterialInstance (Variables|Default|Gety_neg) 0 0 "None" :!class /Script/Engine.PrimitiveComponent))
  (Variables|Materials|SetYNegMat _returnvalue_3)
  (bind _returnvalue_4 (Rendering|Material|CreateDynamicMaterialInstance (Variables|Default|Gety_pos) 0 0 "None" :!class /Script/Engine.PrimitiveComponent))
  (Variables|Materials|SetYPosMat _returnvalue_4)
  (bind _returnvalue_5 (Rendering|Material|CreateDynamicMaterialInstance (Variables|Default|Getz_neg) 0 0 "None" :!class /Script/Engine.PrimitiveComponent))
  (Variables|Materials|SetZNegMat _returnvalue_5)
  (bind _returnvalue_6 (Rendering|Material|CreateDynamicMaterialInstance (Variables|Default|Getz_pos) 0 0 "None" :!class /Script/Engine.PrimitiveComponent))
  (Variables|Materials|SetZPosMat _returnvalue_6))

(fn SetTexture
  (params (X%20Neg :type Texture%202D%20Object%20Reference) (Y%20Neg :type Texture%202D%20Object%20Reference) (Z%20Neg :type Texture%202D%20Object%20Reference) (X%20Pos :type Texture%202D%20Object%20Reference) (Y%20Pos :type Texture%202D%20Object%20Reference) (Z%20Pos :type Texture%202D%20Object%20Reference))
  ;[1 1 1] Set textures inside the created material instances
  (Rendering|Material|SetTextureParameterValue (Variables|Materials|GetXNegMat) "Texture" X%20Neg)
  (Rendering|Material|SetTextureParameterValue (Variables|Materials|GetXPosMat) "Texture" X%20Pos)
  (Rendering|Material|SetTextureParameterValue (Variables|Materials|GetYNegMat) "Texture" Y%20Neg)
  (Rendering|Material|SetTextureParameterValue (Variables|Materials|GetYPosMat) "Texture" Y%20Pos)
  (Rendering|Material|SetTextureParameterValue (Variables|Materials|GetZNegMat) "Texture" Z%20Neg)
  (Rendering|Material|SetTextureParameterValue (Variables|Materials|GetZPosMat) "Texture" Z%20Pos)
  (Rendering|Material|SetScalarParameterValue (Variables|Materials|GetXNegMat) "Brightness" (Variables|Properties|GetBrightness) :!class /Script/Engine.MaterialInstanceDynamic))

(fn SetTextures
  (CallFunction|SetTexture "/Game/SpaceSkyboxes/Textures/ESO349-31/T_ESO349-31_neg_x.T_ESO349-31_neg_x" "/Game/SpaceSkyboxes/Textures/ESO349-31/T_ESO349-31_neg_y.T_ESO349-31_neg_y" "/Game/SpaceSkyboxes/Textures/ESO349-31/T_ESO349-31_neg_z.T_ESO349-31_neg_z" "/Game/SpaceSkyboxes/Textures/ESO349-31/T_ESO349-31_pos_x.T_ESO349-31_pos_x" "/Game/SpaceSkyboxes/Textures/ESO349-31/T_ESO349-31_pos_y.T_ESO349-31_pos_y" "/Game/SpaceSkyboxes/Textures/ESO349-31/T_ESO349-31_pos_z.T_ESO349-31_pos_z"))